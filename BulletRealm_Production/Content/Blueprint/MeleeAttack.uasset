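; MeleeAttack is a short-lived hitbox actor for melee strikes, destroying itself after a 0.001-second delay.
; Overlapping a non-owner character plays a camera shake, then ServerMeleeAttack once applies damage, using the victim's MeleeDamage, and launches it along the owner's forward vector.
; Overlapping the owner only records it as Attacker, the damage causer.
; Box hits spawn a SprintRadialForce at the impact point, intended for wall damage.
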(event OnComponentBeginOverlap(Box)
  (params (OverlappedComponent :type Primitive%20Component%20Object%20Reference) (OtherActor :type Actor%20Object%20Reference) (OtherComp :type Primitive%20Component%20Object%20Reference) (OtherBodyIndex :type Integer) (bFromSweep :type Boolean) (SweepResult :type Hit%20Result%20Structure%20%28by%20ref%29))
  ;[1 1 1] Apply 50 damage (Not bleeding) (Hasan)
  (bind _ascharacter_generic (Utilities|Casting|CastToCharacter_Generic OtherActor))
  (if (== (Components|GetOwner) _ascharacter_generic)
    (Variables|Default|SetAttacker _ascharacter_generic)
    (else
      (Camera|PlayWorldCameraShake "/Game/Blueprint/CameraShakes/MeleeCameraShake.MeleeCameraShake_C" (Transformation|GetWorldLocation (Variables|/Game/Blueprint/Character_Generic.Character_Generic_C|GetFPSCamera _ascharacter_generic)) 0.0 5e+01 1.0 true)
      (CallFunction|ServerMeleeAttack OtherActor))))

(event OnComponentHit(Box)
  (params (HitComponent :type Primitive%20Component%20Object%20Reference) (OtherActor :type Actor%20Object%20Reference) (OtherComp :type Primitive%20Component%20Object%20Reference) (NormalImpulse :type Vector :default "0, 0, 0") (Hit :type Hit%20Result%20Structure%20%28by%20ref%29))
  ;[0.3806 1 0.3146] Apply damage to wall , Done by Hasan
  (Game|SpawnActorfromClass "/Game/Blueprint/SprintRadialForce.SprintRadialForce_C" (Math|Transform|MakeTransform (.location Hit)) "Undefined" 0 0))

(event Custom|ServerMeleeAttack
  (params (otherActor :type Actor%20Object%20Reference))
  ;[1 1 1] Apply 50 damage (Not bleeding) (Hasan)
  (bind _ascharacter_generic (Utilities|Casting|CastToCharacter_Generic otherActor))
  (Utilities|FlowControl|DoOnce false
    (:Completed
      (Game|Damage|ApplyDamage _ascharacter_generic (Variables|/Game/Blueprint/Character_Generic.Character_Generic_C|GetMeleeDamage _ascharacter_generic) (Variables|Default|GetControllerRef) (Variables|Default|GetAttacker) "/Script/Engine.DamageType")
      ;;[1 1 1] Push Back
      (Character|LaunchCharacter _ascharacter_generic (* (Transformation|GetActorForwardVector (Components|GetOwner)) (Variables|Default|GetpushBack)) true true))))

(event EventBeginPlay
  ;[1 1 1] Destroys after 10 miliseconds
  (Utilities|FlowControl|Delay 0.001)
  (Actor|DestroyActor))

(fn ConstructionScript)