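; Generic HUD that draws a first-person crosshair at the screen center, shifted by X and Y adjustment offsets.
; Each DrawHUD casts the player pawn to Character_Generic, caches it and registers itself as that character's HUDRef.
; After a short Delay inside the draw event, it writes the adjusted center coordinates to CenterX and CenterY on the owning PlayerController_Generic's CharacterBP.
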(event EventDrawHUD
  (params (SizeX :type Integer) (SizeY :type Integer))
  (bind _returnvalue (/ SizeX 2))
  (bind _returnvalue_2 (/ SizeY 2))
  (bind _xadjustment (Variables|Default|GetxAdjustment))
  (bind _yadjustment (Variables|Default|GetyAdjustment))
  (bind _returnvalue_3 (- _returnvalue _xadjustment))
  (bind _returnvalue_4 (- _returnvalue_2 _yadjustment))
  (bind _returnvalue_5 (Math|Conversions|ToFloat(Integer) _returnvalue_3))
  (bind _returnvalue_6 (Math|Conversions|ToFloat(Integer) _returnvalue_4))
  ;[1 1 1] Draw crosshair in center of screen, by Saeed
  (bind _ascharacter_generic (Utilities|Casting|CastToCharacter_Generic (Game|GetPlayerCharacter 0)))
  (Utilities|IsValid _ascharacter_generic
    (:Is%20Valid
      (bind _output_get (Variables|Default|SetCharRef _ascharacter_generic))
      (Variables|/Game/Blueprint/Character_Generic.Character_Generic_C|SetHUDRef _output_get self)
      (Canvas|DrawTexture "/Game/Texture/FirstPersonCrosshair.FirstPersonCrosshair" _returnvalue_5 _returnvalue_6 16.0 16.0 0.0 0.0 1.0 1.0 (Utilities|Struct|MakeLinearColor 1.0 1.0 1.0 1.0) "BLEND_Translucent" 1.0 true)
      (Utilities|FlowControl|Delay 0.8)
      (bind _asplayer_controller_generic (Utilities|Casting|CastToPlayerController_Generic (Game|Player|GetOwningPlayerController)))
      (Utilities|IsValid (Variables|/Game/Blueprint/PlayerController_Generic.PlayerController_Generic_C|GetCharacterBP _asplayer_controller_generic)
        (:Is%20Valid
          (Variables|/Game/Blueprint/Character_Generic.Character_Generic_C|SetCenterX (Variables|/Game/Blueprint/PlayerController_Generic.PlayerController_Generic_C|GetCharacterBP _asplayer_controller_generic) _returnvalue_5)
          (Variables|/Game/Blueprint/Character_Generic.Character_Generic_C|SetCenterY (Variables|/Game/Blueprint/PlayerController_Generic.PlayerController_Generic_C|GetCharacterBP _asplayer_controller_generic) _returnvalue_6))))))

(fn ConstructionScript)