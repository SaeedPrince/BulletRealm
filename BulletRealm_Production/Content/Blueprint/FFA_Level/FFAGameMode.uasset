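; FFA game mode that runs the multiplayer lobby and launches the match.
; On login it reads server settings from the game instance, sets up the player's lobby menu and spawns a generic character at a random PlayerStart; SwapCharacter respawns them as the selected class.
; Joins and logouts rebuild the player list and push it to every controller.
; When the ready count reaches max players, it shows a loading screen, waits, then server-travels to Map_E1M1.
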(event Custom|RespawnPlayer
  (params (PlayerController :type Player%20Controller%20Object%20Reference))
  (bind _returnvalue (Pawn|GetControlledPawn PlayerController))
  (bind _spawnpoints (Variables|ServerSettings|GetSpawnPoints))
  ;[0.3563 1 0.1558] Spawn the player as character generic when arriving at lobby menu / tell clients to update their lobby
  (Utilities|IsValid _returnvalue
    (:Is%20Valid
      (Actor|DestroyActor _returnvalue))
    (:Is%20Not%20Valid
      _))
  (bind _returnvalue_2 (Game|SpawnActorfromClass "/Game/Blueprint/Character_Generic.Character_Generic_C" (Transformation|GetActorTransform (Utilities|Array|Get(acopy) _spawnpoints (Math|Random|RandomIntegerinRange 0 (- (Utilities|Array|Length _spawnpoints) 1)))) "Undefined" 0 0))
  (Pawn|Possess PlayerController _returnvalue_2)
  (CallFunction|EveryoneUpdate))

(event Custom|PlayersNotReady
  ;[0.1062 0.2026 1] Player Ready / Start Match
  (bind _result (Math|Integer|DecrementInt (Variables|Default|GetvalueIncDec))
    (:%20%20
      (Variables|Default|SetMatchCount _result))))

(event Custom|EveryoneUpdate
  (bind _allplayercontrollers (Variables|ServerSettings|GetAllPlayerControllers))
  ;[0.09423 1 0.1002] Update all connected players lobby
  (bind _output_get (Variables|ServerSettings|SetCurrentPlayers (Utilities|Array|Length (Variables|ServerSettings|GetAllPlayerControllers))))
  (if (> _output_get 0)
    (Utilities|Array|Clear (Variables|ServerSettings|GetConnectedPlayers))
    (for _array_element _allplayercontrollers
      (bind _asffaplayer_controller (Utilities|Casting|CastToFFAPlayerController _array_element))
      (Utilities|Array|Add (Variables|ServerSettings|GetConnectedPlayers) (Variables|/Game/Blueprint/FFA_Level/FFAPlayerController.FFAPlayerController_C|GetPlayerSettings _asffaplayer_controller))
      (Default|UpdateNumberOfPlayers _asffaplayer_controller (Variables|ServerSettings|GetCurrentPlayers) (Variables|ServerSettings|GetMaxPlayers)))
    (for _array_element_2 _allplayercontrollers
      (bind _asffaplayer_controller_2 (Utilities|Casting|CastToFFAPlayerController _array_element_2))
      (Default|AddPlayerInfo _asffaplayer_controller_2 (Variables|ServerSettings|GetConnectedPlayers)))))

(event Custom|SwapCharacter
  (params (PlayerController :type FFA%20Player%20Controller%20Object%20Reference) (CharacterClass :type Character%20Class%20Reference) (ChangedStatus :type Boolean))
  (bind _returnvalue (Pawn|GetControlledPawn PlayerController))
  (bind _spawnpoints (Variables|ServerSettings|GetSpawnPoints))
  ;[0.1168 1 0.08209] Change default character with the selected character from select screen - characters are falling cause i dont have a level to support. need to check it later
  (if (not ChangedStatus)
    (Utilities|IsValid _returnvalue
      (:Is%20Valid
        (Actor|DestroyActor _returnvalue))
      (:Is%20Not%20Valid
        _))
    (bind _returnvalue_2 (Game|SpawnActorfromClass CharacterClass (Transformation|GetActorTransform (Utilities|Array|Get(acopy) _spawnpoints (Math|Random|RandomIntegerinRange 0 (- (Utilities|Array|Length _spawnpoints) 1)))) "Undefined" 0 0))
    (Pawn|Possess PlayerController _returnvalue_2)))

(event Custom|PlayersReady
  (bind _returnvalue (Game|GetPlayerController 0))
  ;[0.1062 0.2026 1] Player Ready / Start Match
  (bind _result (Math|Integer|IncrementInt (Variables|Default|GetvalueIncDec))
    (:%20%20
      (bind _output_get (Variables|Default|SetMatchCount _result))
      (bind _asthe_game_instance (Utilities|Casting|CastTotheGameInstance (Game|GetGameInstance)))
      (if (== _output_get (Variables|/Game/Blueprint/AllLevels/theGameInstance.theGameInstance_C|GetMaxPlayer _asthe_game_instance))
        ;;[1 1 1] Adding loading screen tempo
        (bind _asffaplayer_controller (Utilities|Casting|CastToFFAPlayerController (Game|GetPlayerController 0)))
        (Default|ShowLoadingScreenonServer _asffaplayer_controller)
        (Utilities|FlowControl|Delay 12.5)
        (Input|SetInputModeGameOnly _returnvalue)
        (Development|ExecuteConsoleCommand "servertravel Map_E1M1" _returnvalue)))))

(event EventOnLogout
  (params (ExitingController :type Controller%20Object%20Reference))
  (bind _allplayercontrollers (Variables|ServerSettings|GetAllPlayerControllers))
  ;[1 1 1] Remove player controllers connected and informations in each player lobby instance
  (bind (_array_element _array_index) (Utilities|Array|ForEachLoopwithBreak _allplayercontrollers :!label _label)
    (:LoopBody
      (if (== _array_element ExitingController)
        (goto _label Break)))
    (:Completed
      (Utilities|Array|RemoveIndex _allplayercontrollers _array_index)
      (Utilities|Array|RemoveIndex (Variables|ServerSettings|GetConnectedPlayers) _array_index)
      (CallFunction|EveryoneUpdate))))

(event EventPostLogin
  (params (NewPlayer :type Player%20Controller%20Object%20Reference))
  ;[0.1779 1 0.1195] Initial Setup oocurs of Event Post Login
  (Networking|SwitchHasAuthority
    (:Authority
      (Utilities|Array|Add (Variables|ServerSettings|GetAllPlayerControllers) NewPlayer)
      (bind _outactors (Actor|GetAllActorsOfClass "/Script/Engine.PlayerStart"))
      (Variables|ServerSettings|SetSpawnPoints _outactors)
      (bind _asthe_game_instance (Utilities|Casting|CastTotheGameInstance (Game|GetGameInstance)))
      (Variables|ServerSettings|SetServerName (Variables|/Game/Blueprint/AllLevels/theGameInstance.theGameInstance_C|GetServerName _asthe_game_instance))
      (Variables|ServerSettings|SetMaxPlayers (Variables|/Game/Blueprint/AllLevels/theGameInstance.theGameInstance_C|GetMaxPlayer _asthe_game_instance))
      (Variables|Default|SetPlayerName (Variables|/Game/Blueprint/AllLevels/theGameInstance.theGameInstance_C|GetPlayerName _asthe_game_instance))
      (bind _asffaplayer_controller (Utilities|Casting|CastToFFAPlayerController NewPlayer))
      (bind _output_get (Variables|ServerSettings|SetFFAPlayerControllerRef _asffaplayer_controller))
      (Default|InitialSetup _output_get)
      (Default|SetupLobbyMenu (Variables|ServerSettings|GetFFAPlayerControllerRef) (Variables|ServerSettings|GetServerName))
      (CallFunction|RespawnPlayer (Variables|ServerSettings|GetFFAPlayerControllerRef)))))

(fn ConstructionScript)