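; Smoke bomb actor that runs a timed smoke effect with Wwise audio, then destroys itself.
; BeginPlay chains delays to start the sound and particle system, end its trails after about 15 seconds, swap to a tail sound, and clean up.
; An IsAlreadyDamaged helper searches the DamagedActors array, but nothing in this graph calls it or applies damage.
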(event EventBeginPlay
  (bind _self self)
  (bind _particlesystem (Variables|Default|GetParticleSystem))
  (Utilities|FlowControl|Delay 1.0)
  (Class|AkGameplayStatics|PostEvent "/Game/SoundWave/SFX/Weapons/Equip/Play_SFX_SmokeGrenade.Play_SFX_SmokeGrenade" self true)
  (Components|Activation|Activate _particlesystem false)
  (Utilities|FlowControl|Delay 15.0)
  (Effects|Particles|Trails|EndTrails _particlesystem)
  (Utilities|FlowControl|Delay 4.0)
  (Class|AkGameplayStatics|PostEvent "/Game/SoundWave/SFX/Weapons/Equip/Stop_SFX_SmokeGrenade.Stop_SFX_SmokeGrenade" _self false)
  (Class|AkGameplayStatics|PostEvent "/Game/SoundWave/SFX/Weapons/Equip/Play_SFX_SmokeGrenadeTail.Play_SFX_SmokeGrenadeTail" _self false)
  (Utilities|FlowControl|Delay 3.0)
  (Actor|DestroyActor))

(fn ConstructionScript)

(fn IsAlreadyDamaged
  (params (ActorInput :type Actor%20Object%20Reference))
  (bind _array_element (Utilities|Array|ForEachLoopwithBreak (Variables|Hit|GetDamagedActors) :!label _label)
    (:LoopBody
      (if (== _array_element ActorInput)
        (LocalVariables|SetResult true)
        (goto _label Break)
        (else
          (LocalVariables|SetResult false))))
    (:Completed
      (return (LocalVariables|GetResult)))))