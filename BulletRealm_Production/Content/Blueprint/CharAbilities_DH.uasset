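; Character component that handles shooter combat feedback: first/third-person animations, muzzle and casing particles, and Wwise sound and voice-over.
; BeginPlay caches character, controller and anim Blueprints; action events mostly route through Server and Multicast events to those targets.
; Tick uses DoOnce gates to toggle low health/stamina audio and HUD warnings and trigger the Overseer's last-30-seconds line.
; Aiming hides the first-person mesh and reattaches the gun to the camera, adjusting sensitivity and walk speed.
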(event Custom|BulletFireLoopSound
  ;[0 0.1896 1] Sounds
  ;;[0 0.1896 1] Begin Fire(when fire is pressed play particles and sounds)
  (CallFunction|ServerBulletLoop))

(event Custom|BulletFireTailSound
  ;[0 0.1896 1] Sounds
  ;;[0 0.1896 1] Fire release (if fire is released stop particles and tail SFX)
  (CallFunction|StopFireLoopMontageMulticast))

(event Custom|ServerCookGrenade
  ;[0 1 1] Animations
  ;;[1 1 1] Cook Grenade
  (CallFunction|MulticastCookGrenade))

(event Custom|DeathSound
  ;[0 0.1896 1] Sounds
  ;;[0 0.1912 1] Death Sound
  (CallFunction|ServerDeathSound))

(event Custom|ServerDeathSound
  ;[0 0.1896 1] Sounds
  ;;[0 0.1912 1] Death Sound
  (CallFunction|MulticastDeathSound))

(event Custom|HittingAnEnemySound
  ;[0 0.1896 1] Sounds
  ;;[0 0.1912 1] Hitting an Enemy Sound
  (Class|AkGameplayStatics|PostEvent "/Game/SoundWave/SFX/Actions/Play_SFX_HittingEnemy.Play_SFX_HittingEnemy" (Game|GetPlayerCharacter 0) false))

(event Custom|MulticastCookGrenade
  ;[0 1 1] Animations
  ;;[1 1 1] Cook Grenade
  (Default|CookGrenade (Variables|Default|GetTPP_AnimationBP))
  (Default|GrenadeCookFPP (Variables|Default|GetFPP_Animation)))

(event Custom|OverseerHeadshotSound
  ;[0 0.1896 1] Sounds
  ;;[0 0.1912 1] Headshot
  (Utilities|FlowControl|Delay 0.2)
  (Utilities|FlowControl|DoOnce false :!label _label
    (:Completed
      (Class|AkGameplayStatics|PostEvent "/Game/SoundWave/VO/Overseer/Play_VO_Overseer_HeadShot.Play_VO_Overseer_HeadShot" (Game|GetPlayerCharacter 0) false)
      (Utilities|FlowControl|Delay 1.3)
      (goto _label Reset))))

(event Custom|BulletCasingBounceSound
  (params (ActorRef :type Actor%20Object%20Reference))
  ;[0 0.1896 1] Sounds
  ;;[0 0.1896 1] Bullet Casing Bounce Sound
  (CallFunction|ServerBulletCasingBounce))

(event Custom|MulticastDeathSound
  ;[0 0.1896 1] Sounds
  ;;[0 0.1912 1] Death Sound
  (Class|AkGameplayStatics|PostEvent "/Game/SoundWave/VO/Marc/Play_VO_Marc_Death.Play_VO_Marc_Death" (Game|GetPlayerCharacter 0) true))

(event Custom|LowHealthSound
  ;[0 0.1896 1] Sounds
  ;;[0 0.1912 1] Low Health Sounds
  (Class|AkGameplayStatics|PostEvent "/Game/SoundWave/SFX/Actions/Play_SFX_LowHealth.Play_SFX_LowHealth" (Game|GetPlayerCharacter 0) false))

(event Custom|ServerBulletCasingBounce
  ;[0 0.1896 1] Sounds
  ;;[0 0.1896 1] Bullet Casing Bounce Sound
  (Utilities|FlowControl|Delay (Math|Random|RandomFloatinRange 0.3 0.5))
  (CallFunction|MulticastBulletCasingBounce))

(event Custom|MeleeMontageMulticast
  ;[0 1 1] Animations
  ;;[1 1 1] Start Melee Montage
  ;;;[1 1 1] Melee
  (Default|MelleAttack (Variables|Default|GetTPP_AnimationBP))
  (Default|MeleeAttackFPP (Variables|Default|GetFPP_Animation)))

(event Custom|OverseerLast30SecondsSound
  ;[0 0.1896 1] Sounds
  ;;[0 0.1912 1] Final 30 seconds
  (Class|AkGameplayStatics|PostEvent "/Game/SoundWave/VO/Overseer/Play_VO_Overseer_Last30.Play_VO_Overseer_Last30" (Game|GetPlayerCharacter 0) false))

(event Custom|BeginMuzzleParticle
  (params (Which%20Particle%20To%20Start%20FPP :type Actor%20Component%20Object%20Reference) (Charcter :type Character%20Generic%20Object%20Reference) (Which%20Particle%20To%20Start%20TPP :type Actor%20Component%20Object%20Reference))
  ;[0.2707 0 1] Particles
  ;;[0.2707 0 1] Patrticle Muzzle Flash
  (CallFunction|StartMuzzleFlashParticle Which%20Particle%20To%20Start%20FPP Charcter Which%20Particle%20To%20Start%20TPP))

(event Custom|MulticastStartMuzzleFlashParticle
  (bind _characterrefrence (Variables|Default|GetCharacterRefrence))
  (bind _muzzleflashtpp (Variables|/Game/Blueprint/Character_Generic.Character_Generic_C|GetMuzzleFlashTPP _characterrefrence))
  (bind _currentweapon (Variables|/Game/Blueprint/Character_Generic.Character_Generic_C|GetCurrentWeapon _characterrefrence))
  (bind _particleflash (Utilities|Struct|BreakWeaponStruct _currentweapon))
  (Effects|Components|ParticleSystem|SetTemplate (Variables|/Game/Blueprint/Character_Generic.Character_Generic_C|GetMuzzleFlashFPP _characterrefrence) _particleflash)
  (Effects|Components|ParticleSystem|SetTemplate _muzzleflashtpp _particleflash)
  (Components|Activation|Activate _muzzleflashtpp false))

(event Custom|StartMeleeMontage
  ;[0 1 1] Animations
  ;;[1 1 1] Start Melee Montage
  (CallFunction|ServerStartMeleeMontage))

(event Custom|SmokeGrenadeSound
  (params (Actor%20to%20spawn%20sound :type Actor%20Object%20Reference))
  ;[0 0.1896 1] Sounds
  ;;[0 0.1912 1] Smoke Grenade Sound
  (CallFunction|ServerSmokeGrenadeSound Actor%20to%20spawn%20sound))

(event Custom|MulticastBulletCasingBounce
  ;[0 0.1896 1] Sounds
  ;;[0 0.1896 1] Bullet Casing Bounce Sound
  (Class|AkGameplayStatics|PostEvent (.ShellCasingBounce (Utilities|Struct|BreakWeaponStruct (Variables|/Game/Blueprint/Character_Generic.Character_Generic_C|GetCurrentWeapon (Variables|Default|GetCharacterRefrence)))) (Game|GetPlayerCharacter 0) false))

(event Custom|ServerStartMeleeMontage
  ;[0 1 1] Animations
  ;;[1 1 1] Start Melee Montage
  (CallFunction|MeleeMontageMulticast))

(event Custom|HealingSound
  ;[0 0.1896 1] Sounds
  ;;[0 0.1912 1] Healing sound
  (Class|AkGameplayStatics|PostEvent 0 (Game|GetPlayerCharacter 0) false))

(event Custom|MulticastWeaponFireSound
  (params (ActorRef :type Actor%20Object%20Reference) (ActorLocation :type Vector))
  ;[0 0.1896 1] Sounds
  ;;[0 0.1912 1] Weapon Fire Sound
  (Class|AkGameplayStatics|PostEvent (.FireSound (Utilities|Struct|BreakWeaponStruct (Variables|/Game/Blueprint/Character_Generic.Character_Generic_C|GetCurrentWeapon (Variables|Default|GetCharacterRefrence)))) ActorRef false))

(event Custom|WallDestructionSound
  (params (Location :type Vector))
  ;[0 0.1896 1] Sounds
  ;;[0 0.1912 1] Wall Destruction Sound
  (CallFunction|ServerWallDestructionSound Location))

(event Custom|ReloadingSound
  (bind _returnvalue (Game|GetPlayerCharacter 0))
  ;[0 0.1896 1] Sounds
  ;;[0 0.1912 1] Reloading sound
  (Class|AkGameplayStatics|PostEvent (.ReloadSound (Utilities|Struct|BreakWeaponStruct (Variables|/Game/Blueprint/Character_Generic.Character_Generic_C|GetCurrentWeapon (Variables|Default|GetCharacterRefrence)))) _returnvalue false)
  (Class|AkGameplayStatics|PostEvent "/Game/SoundWave/VO/Marc/Play_VO_Reload_Marc_048a.Play_VO_Reload_Marc_048a" _returnvalue false))

(event Custom|ServerWallDestructionSound
  (params (Location :type Vector))
  ;[0 0.1896 1] Sounds
  ;;[0 0.1912 1] Wall Destruction Sound
  (Utilities|FlowControl|DoOnce false :!label _label
    (:Completed
      (Class|AkGameplayStatics|PostEventatLocation "/Game/SoundWave/SFX/Actions/Play_SFX_WallDestruction.Play_SFX_WallDestruction" Location "0, 0, 0")
      (Utilities|FlowControl|Delay 1.0)
      (goto _label Reset))))

(event Custom|SelectGrenade
  ;[0 1 1] Animations
  (Default|GrenadeSelected (Variables|Default|GetTPP_AnimationBP))
  (Default|GrenadeSelectedFPP (Variables|Default|GetFPP_Animation)))

(event Custom|ServerWeaponFIre
  (params (ActorRef :type Actor%20Object%20Reference) (ActorLocation :type Vector))
  ;[0 0.1896 1] Sounds
  ;;[0 0.1912 1] Weapon Fire Sound
  (CallFunction|MulticastWeaponFireSound ActorRef ActorLocation))

(event Custom|StopOutOfBreath
  ;[0 0.1896 1] Sounds
  ;;[0 0.1912 1] Out Of Breath Sound
  (Class|AkGameplayStatics|PostEvent "/Game/SoundWave/VO/Marc/Stop_VO_Breaths_Marc_052a.Stop_VO_Breaths_Marc_052a" (Game|GetPlayerCharacter 0) false))

(event Custom|HUDStaminaShow
  ;[0 1 1] Animations
  ;;[1 1 1] HUD Stamina Low Feedback
  (Default|HUDStaminaOut (Variables|/Game/Blueprint/Character_Generic.Character_Generic_C|GetCharAbilities_TB (Variables|Default|GetCharacterRefrence))))

(event Custom|EndMuzzleParticle
  (params (Which%20Particle%20to%20End :type Actor%20Component%20Object%20Reference) (Charcter :type Character%20Generic%20Object%20Reference))
  ;[0.2707 0 1] Particles
  ;;[0.2707 0 1] Patrticle Muzzle Flash
  (CallFunction|StopMuzzleFlashParticle Which%20Particle%20to%20End Charcter))

(event Custom|EmptyAKSound
  (bind _characterrefrence (Variables|Default|GetCharacterRefrence))
  ;[0 0.1896 1] Sounds
  ;;[0 0.1896 1] Empty AK Sound
  (if (<= (.AmmoInMag (Utilities|Struct|BreakWeaponStruct (Variables|/Game/Blueprint/Character_Generic.Character_Generic_C|GetCurrentWeapon _characterrefrence))) 0)
    (Class|AkGameplayStatics|PostEvent "/Game/SoundWave/SFX/Weapons/AK47/Play_SFX_AK47_Empty.Play_SFX_AK47_Empty" _characterrefrence false)))

(event Custom|ReloadMontageMulticast
  ;[0 1 1] Animations
  ;;[1 1 1] Reloading
  ;;;[1 1 1] Reload
  (Default|ReloadWeapon (Variables|Default|GetTPP_AnimationBP))
  (Default|ReloadWeaponFPP (Variables|Default|GetFPP_Animation)))

(event Custom|MulticastStartHealing
  ;[0 1 1] Animations
  ;;[1 1 1] Healing
  (Default|Healing (Variables|Default|GetTPP_AnimationBP))
  (Default|HealingFPP (Variables|Default|GetFPP_Animation)))

(event Custom|ServerSmokeGrenadeSound
  (params (Actor%20to%20spawn%20sound :type Actor%20Object%20Reference))
  ;[0 0.1896 1] Sounds
  ;;[0 0.1912 1] Smoke Grenade Sound
  (CallFunction|MulticastSmokeGrenadeSound Actor%20to%20spawn%20sound))

(event Custom|ThrowGrenade
  ;[0 1 1] Animations
  ;;[1 1 1] Throw Grenade
  (CallFunction|ServerThrowGrenade))

(event Custom|StopFireLoopMontageMulticast
  ;[0 1 1] Animations
  ;;[1 1 1] Stop
  (Default|AimFireLoopStop (Variables|Default|GetTPP_AnimationBP))
  (Default|AimFireLoopStopFPP (Variables|Default|GetFPP_Animation)))

(event Custom|ServerThrowGrenade
  ;[0 1 1] Animations
  ;;[1 1 1] Throw Grenade
  (CallFunction|MulticastThrowGrenade))

(event Custom|MulticastHitSound
  ;[0 0.1896 1] Sounds
  ;;[0 0.1912 1] Getting Hit Sound
  (Class|AkGameplayStatics|PostEvent "/Game/SoundWave/VO/Marc/Play_VO_Marc_RandomHit.Play_VO_Marc_RandomHit" (Game|GetPlayerCharacter 0) false))

(event Custom|MulticastThrowGrenade
  ;[0 1 1] Animations
  ;;[1 1 1] Throw Grenade
  (Default|ThrowGrenade (Variables|Default|GetTPP_AnimationBP))
  (Default|GrenadeThrowFPP (Variables|Default|GetFPP_Animation)))

(event Custom|StartHealing
  ;[0 1 1] Animations
  ;;[1 1 1] Healing
  (CallFunction|ServerStartHealing))

(event Custom|MulticastStartcasingParticle
  (bind _characterrefrence (Variables|Default|GetCharacterRefrence))
  (bind _currentweapon (Variables|/Game/Blueprint/Character_Generic.Character_Generic_C|GetCurrentWeapon _characterrefrence))
  (bind _bulletcasingejecttpp (Variables|/Game/Blueprint/Character_Generic.Character_Generic_C|GetBulletCasingEjectTPP _characterrefrence))
  (bind _particlecasing (Utilities|Struct|BreakWeaponStruct _currentweapon))
  ;[1 1 1] casing eject
  (Effects|Components|ParticleSystem|SetTemplate (Variables|/Game/Blueprint/Character_Generic.Character_Generic_C|GetBulletCasingEjectFPP _characterrefrence) _particlecasing)
  (Effects|Components|ParticleSystem|SetTemplate _bulletcasingejecttpp _particlecasing)
  (Components|Activation|Activate _bulletcasingejecttpp false))

(event Custom|MulticastCasingParticle
  (bind _characterrefrence (Variables|Default|GetCharacterRefrence))
  (CallFunction|BeginCasingParticle (Variables|/Game/Blueprint/Character_Generic.Character_Generic_C|GetBulletCasingEjectFPP _characterrefrence) _characterrefrence (Variables|/Game/Blueprint/Character_Generic.Character_Generic_C|GetBulletCasingEjectTPP _characterrefrence)))

(event Custom|GrenadeThrowSound
  ;[0 0.1896 1] Sounds
  ;;[0 0.1912 1] Throw Grenade VO
  (Class|AkGameplayStatics|PostEvent "/Game/SoundWave/VO/Marc/Play_VO_Marc_RandomEquipment.Play_VO_Marc_RandomEquipment" (Game|GetPlayerCharacter 0) true))

(event Custom|SnapGuntoCamera
  (bind _characterrefrence (Variables|Default|GetCharacterRefrence))
  (bind _gun_fpp (Variables|/Game/Blueprint/Character_Generic.Character_Generic_C|GetGUN_FPP _characterrefrence))
  ;[1 1 1] Snap  Gun to Camera/Snap Gun to Mesh
  (Rendering|SetVisibility (Variables|/Game/Blueprint/Character_Generic.Character_Generic_C|GetFPP _characterrefrence) false false)
  (Transformation|DetachFromComponent _gun_fpp "KeepRelative" "KeepRelative" "KeepRelative" true)
  (Transformation|AttachComponentToComponent _gun_fpp (Variables|/Game/Blueprint/Character_Generic.Character_Generic_C|GetAim_Camera _characterrefrence) "None" "KeepRelative" "KeepRelative" "KeepRelative" true)
  (Transformation|SetRelativeLocationAndRotation _gun_fpp "-15.000000,0.700000,-15.500000" "0.000000,-90.000000,-0.500000" false false)
  (Variables|/Game/Blueprint/Character_Generic.Character_Generic_C|SetMouseSensitivityYaw _characterrefrence 3.0)
  (Variables|/Game/Blueprint/Character_Generic.Character_Generic_C|SetMouseSensitivityPitch _characterrefrence 2.0)
  (if (not (Variables|/Game/Blueprint/Character_Generic.Character_Generic_C|GetIsCrouching _characterrefrence))
    (Variables|/Script/Engine.CharacterMovementComponent|SetMaxWalkSpeed (Variables|/Script/Engine.Character|GetCharacterMovement _characterrefrence) (Variables|/Game/Blueprint/Character_Generic.Character_Generic_C|GetDefaultAimSpeed _characterrefrence))))

(event Custom|StartReloadAK
  ;[0 1 1] Animations
  ;;[1 1 1] Reloading
  (CallFunction|ServerAKReload))

(event Custom|MulticastSmokeGrenadeSound
  (params (Actor%20to%20spawn%20sound :type Actor%20Object%20Reference))
  ;[0 0.1896 1] Sounds
  ;;[0 0.1912 1] Smoke Grenade Sound
  (Class|AkGameplayStatics|PostEvent "/Game/SoundWave/SFX/Weapons/Equip/Play_SFX_SmokeGrenade.Play_SFX_SmokeGrenade" Actor%20to%20spawn%20sound true))

(event Custom|ServerGrenadeThrowSound
  ;[0 0.1896 1] Sounds
  ;;[0 0.1912 1] Throw Grenade VO
  (CallFunction|MulticastGrenadeThrowSound))

(event Custom|ServerAKReload
  ;[0 1 1] Animations
  ;;[1 1 1] Reloading
  (CallFunction|ReloadMontageMulticast))

(event Custom|ServerStartHealing
  ;[0 1 1] Animations
  ;;[1 1 1] Healing
  (CallFunction|MulticastStartHealing))

(event Custom|MulticastGrenadeThrowSound
  ;[0 0.1896 1] Sounds
  ;;[0 0.1912 1] Throw Grenade VO
  (Class|AkGameplayStatics|PostEvent "/Game/SoundWave/VO/Marc/Play_VO_Marc_RandomEquipment.Play_VO_Marc_RandomEquipment" (Game|GetPlayerCharacter 0) true))

(event Custom|ServerBulletLoop
  (bind _characterrefrence (Variables|Default|GetCharacterRefrence))
  ;[0 0.1896 1] Sounds
  ;;[0 0.1896 1] Begin Fire(when fire is pressed play particles and sounds)
  (if (<= (.AmmoInMag (Utilities|Struct|BreakWeaponStruct (Variables|/Game/Blueprint/Character_Generic.Character_Generic_C|GetCurrentWeapon (Variables|Default|GetCharacterRefrence)))) 0)
    (CallFunction|EmptyAKSound)
    (elif (Variables|/Game/Blueprint/Character_Generic.Character_Generic_C|GetIsFiring _characterrefrence)
      (if (Variables|/Game/Blueprint/Character_Generic.Character_Generic_C|GetIsAiming _characterrefrence)
        (CallFunction|FireLoopMontageMulticast)
        (else
          (CallFunction|HipFireLoopMontageMulticast))))))

(event Custom|HipFireLoopMontageMulticast
  ;[0 1 1] Animations
  ;;[1 1 1] Fire
  (Default|HipFireLoop (Variables|Default|GetTPP_AnimationBP))
  (Default|HipFireLoopFPP (Variables|Default|GetFPP_Animation)))

(event Custom|ServerHitSound
  ;[0 0.1896 1] Sounds
  ;;[0 0.1912 1] Getting Hit Sound
  (CallFunction|MulticastHitSound))

(event Custom|BeginCasingParticle
  (params (Which%20particle%20to%20start%20FPP :type Actor%20Component%20Object%20Reference) (Charcter :type Character%20Generic%20Object%20Reference) (Which%20particle%20to%20start%20TPP :type Actor%20Component%20Object%20Reference))
  ;[0.2707 0 1] Particles
  ;;[0.2707 0 1] Particle Casing Eject
  (CallFunction|StartCasingParticle Which%20particle%20to%20start%20FPP Charcter Which%20particle%20to%20start%20TPP))

(event Custom|EndCasingParticle
  (params (Which%20Particle%20To%20End :type Actor%20Component%20Object%20Reference) (Character :type Character%20Generic%20Object%20Reference))
  ;[0.2707 0 1] Particles
  ;;[0.2707 0 1] Particle Casing Eject
  (CallFunction|StopCasingParticle Which%20Particle%20To%20End Character))

(event Custom|FootStepSound
  (params (Actor%20to%20spawn%20sound :type Actor%20Object%20Reference))
  ;[0 0.1896 1] Sounds
  ;;[0 0.1912 1] Foot Step Sound
  (Class|AkGameplayStatics|PostEvent "/Game/SoundWave/SFX/Actions/Play_SFX_FootStep.Play_SFX_FootStep" Actor%20to%20spawn%20sound false))

(event Custom|SnapGuntoFPPMesh
  (bind _characterrefrence (Variables|Default|GetCharacterRefrence))
  (bind _characterrefrence_2 (Variables|Default|GetCharacterRefrence))
  (bind _gun_fpp (Variables|/Game/Blueprint/Character_Generic.Character_Generic_C|GetGUN_FPP _characterrefrence))
  ;[1 1 1] Snap  Gun to Camera/Snap Gun to Mesh
  (Rendering|SetVisibility (Variables|/Game/Blueprint/Character_Generic.Character_Generic_C|GetFPP _characterrefrence_2) true false)
  (Transformation|DetachFromComponent _gun_fpp "KeepRelative" "KeepRelative" "KeepRelative" true)
  (Transformation|AttachComponentToComponent _gun_fpp (Variables|/Game/Blueprint/Character_Generic.Character_Generic_C|GetFPP _characterrefrence) "Gun" "KeepRelative" "KeepRelative" "KeepRelative" true)
  (Transformation|SetRelativeLocationAndRotation (Variables|/Game/Blueprint/Character_Generic.Character_Generic_C|GetGUN_FPP _characterrefrence_2) "0, 0, 0" (Variables|Default|GetStartRot) false false)
  (Variables|/Game/Blueprint/Character_Generic.Character_Generic_C|SetMouseSensitivityYaw _characterrefrence 1.0)
  (Variables|/Game/Blueprint/Character_Generic.Character_Generic_C|SetMouseSensitivityPitch _characterrefrence 1.0)
  (if (not (Variables|/Game/Blueprint/Character_Generic.Character_Generic_C|GetIsCrouching _characterrefrence))
    (Variables|/Script/Engine.CharacterMovementComponent|SetMaxWalkSpeed (Variables|/Script/Engine.Character|GetCharacterMovement _characterrefrence) (Variables|/Game/Blueprint/Character_Generic.Character_Generic_C|GetDefaultMoveSpeed _characterrefrence))))

(event Custom|ServerFootStepSound
  ;[0 0.1896 1] Sounds
  ;;[0 0.1912 1] Foot Step Sound
  (CallFunction|MulticastFootStepSound))

(event Custom|HUDHealthLowShow
  ;[0 1 1] Animations
  ;;[1 1 1] HUD Health Low Feedback
  (Default|ShowWLowHealth (Variables|/Game/Blueprint/Character_Generic.Character_Generic_C|GetCharAbilities_TB (Variables|Default|GetCharacterRefrence))))

(event Custom|HitSound
  ;[0 0.1896 1] Sounds
  ;;[0 0.1912 1] Getting Hit Sound
  (Class|AkGameplayStatics|PostEvent "/Game/SoundWave/VO/Marc/Play_VO_Marc_RandomHit.Play_VO_Marc_RandomHit" (Game|GetPlayerCharacter 0) false))

(event Custom|FireLoopMontageMulticast
  ;[0 1 1] Animations
  ;;[1 1 1] Fire
  (Default|AimFireLoop (Variables|Default|GetTPP_AnimationBP))
  (Default|AimFireLoopFPP (Variables|Default|GetFPP_Animation)))

(event Custom|MulticastGrenadeExplode
  (params (ActorLocation :type Actor%20Object%20Reference))
  ;[0 0.1896 1] Sounds
  ;;[0 0.1912 1] Grenade Explode
  (Class|AkGameplayStatics|PostEvent "/Game/SoundWave/SFX/Weapons/Equip/Play_SFX_Explode.Play_SFX_Explode" ActorLocation false))

(event Custom|MulticastFootStepSound
  (params (Actor%20to%20spawn%20sound :type Actor%20Object%20Reference))
  ;[0 0.1896 1] Sounds
  ;;[0 0.1912 1] Foot Step Sound
  (Class|AkGameplayStatics|PostEvent "/Game/SoundWave/SFX/Actions/Play_SFX_FootStep.Play_SFX_FootStep" (stale Custom|FootStepSound Actor%20to%20spawn%20sound) false))

(event Custom|OutOfBreathSound
  ;[0 0.1896 1] Sounds
  ;;[0 0.1912 1] Out Of Breath Sound
  (Class|AkGameplayStatics|PostEvent "/Game/SoundWave/VO/Marc/Play_VO_Breaths_Marc_052a.Play_VO_Breaths_Marc_052a" (Game|GetPlayerCharacter 0) false))

(event Custom|OverseerKillSound
  ;[0 0.1896 1] Sounds
  ;;[0 0.1912 1] Kill sound
  (Utilities|FlowControl|DoOnce false :!label _label
    (:Completed
      (Utilities|FlowControl|Delay 1.0)
      (Class|AkGameplayStatics|PostEvent "/Game/SoundWave/VO/Overseer/Play_VO_Overseer_Kill.Play_VO_Overseer_Kill" (Components|GetOwner) false)
      (Utilities|FlowControl|Delay 2.0)
      (goto _label Reset))))

(event Custom|AimMontageMulticast
  ;[0 1 1] Animations
  ;;[1 1 1] Aiming
  ;;;[1 1 1] Aim
  (Default|Aim (Variables|Default|GetTPP_AnimationBP))
  (Default|AimFPP (Variables|Default|GetFPP_Animation)))

(event Custom|HUDStanimaHide
  ;[0 1 1] Animations
  ;;[1 1 1] HUD Stamina Low Feedback
  (Default|HUDStopStaminaOut (Variables|/Game/Blueprint/Character_Generic.Character_Generic_C|GetCharAbilities_TB (Variables|Default|GetCharacterRefrence))))

(event Custom|MulticastMuzzleFlash
  (bind _characterrefrence (Variables|Default|GetCharacterRefrence))
  (CallFunction|BeginMuzzleParticle (Variables|/Game/Blueprint/Character_Generic.Character_Generic_C|GetMuzzleFlashFPP _characterrefrence) _characterrefrence (Variables|/Game/Blueprint/Character_Generic.Character_Generic_C|GetMuzzleFlashTPP _characterrefrence)))

(event Custom|AimingMontage
  ;[0 1 1] Animations
  ;;[1 1 1] Aiming
  (CallFunction|ServerAimingMontage)
  (CallFunction|SnapGuntoCamera))

(event Custom|LowHealthSoundStop
  ;[0 0.1896 1] Sounds
  ;;[0 0.1912 1] Low Health Sounds
  (Class|AkGameplayStatics|PostEvent "/Game/SoundWave/SFX/Actions/Stop_SFX_LowHealth.Stop_SFX_LowHealth" (Game|GetPlayerCharacter 0) false))

(event Custom|Tick
  (params (Frame%20In%20seconds :type Float%20%28single-precision%29))
  (bind _controllerrefrence (Variables|Default|GetControllerRefrence))
  ;[0 1 0.1455] Breath Sounds/Low Stamina Feedback /Heartbeat Low Health
  ;;[1 0 0.8948] Last 30 seconds
  (if (Math|Boolean|ANDBoolean (== (Variables|/Game/Blueprint/PlayerController_Generic.PlayerController_Generic_C|GetPC_minutes _controllerrefrence) 0) (== (Variables|/Game/Blueprint/PlayerController_Generic.PlayerController_Generic_C|GetPC_decimal_seconds _controllerrefrence) 3) (== (Variables|/Game/Blueprint/PlayerController_Generic.PlayerController_Generic_C|GetPC_seconds _controllerrefrence) 0))
    (Utilities|FlowControl|DoOnce false
      (:Completed
        (CallFunction|OverseerLast30SecondsSound)))))

(event Custom|ServerAimingMontage
  ;[0 1 1] Animations
  ;;[1 1 1] Aiming
  (CallFunction|AimMontageMulticast))

(event Custom|HUDHealthLowHide
  ;[0 1 1] Animations
  ;;[1 1 1] HUD Health Low Feedback
  (Default|HideWLowHealth (Variables|/Game/Blueprint/Character_Generic.Character_Generic_C|GetCharAbilities_TB (Variables|Default|GetCharacterRefrence))))

(event Custom|CookGrenade
  ;[0 1 1] Animations
  ;;[1 1 1] Cook Grenade
  (CallFunction|ServerCookGrenade))

(event EventTick
  (params (DeltaSeconds :type Float%20%28single-precision%29))
  (bind _characterrefrence (Variables|Default|GetCharacterRefrence))
  ;[0 1 0.1455] Breath Sounds/Low Stamina Feedback /Heartbeat Low Health
  (Utilities|IsValid (Variables|Default|GetControllerRefrence)
    (:Is%20Valid
      (CallFunction|Tick DeltaSeconds)
      (if (Variables|/Game/Blueprint/Character_Generic.Character_Generic_C|GetIsPlayerDead _characterrefrence)
        ;;[0 0 0] If Dead stop sounds
        (CallFunction|LowHealthSoundStop)
        (CallFunction|StopOutOfBreath)
        (else
          (Utilities|FlowControl|Sequence
            (:then_0
              ;;[1 0 0] Low Health
              (if (<= (Variables|/Game/Blueprint/Character_Generic.Character_Generic_C|GetHealth _characterrefrence) 2e+01)
                (Utilities|FlowControl|Sequence
                  (:then_0
                    (Utilities|FlowControl|DoOnce false :!label _label
                      (:Completed
                        (CallFunction|LowHealthSound)
                        (CallFunction|HUDHealthLowShow))))
                  (:then_1
                    (goto _label_2 Reset)))
                (else
                  (Utilities|FlowControl|Sequence
                    (:then_0
                      (goto _label Reset))
                    (:then_1
                      (Utilities|FlowControl|DoOnce false :!label _label_2
                        (:Completed
                          (CallFunction|LowHealthSoundStop)
                          (CallFunction|HUDHealthLowHide))))))))
            (:then_1
              ;;[0 0.1912 1] Low Stamina
              (if (and (<= (Variables|/Game/Blueprint/Character_Generic.Character_Generic_C|GetStamina _characterrefrence) (Variables|/Game/Blueprint/Character_Generic.Character_Generic_C|GetMinStaminaForSprint _characterrefrence)) (not (Variables|/Game/Blueprint/Character_Generic.Character_Generic_C|GetIsSprinting _characterrefrence)))
                (Utilities|FlowControl|Sequence
                  (:then_0
                    (Utilities|FlowControl|DoOnce false :!label _label_3
                      (:Completed
                        (CallFunction|HUDStaminaShow)
                        (CallFunction|OutOfBreathSound))))
                  (:then_1
                    (goto _label_4 Reset)))
                (else
                  (Utilities|FlowControl|Sequence
                    (:then_0
                      (goto _label_3 Reset))
                    (:then_1
                      (Utilities|FlowControl|DoOnce false :!label _label_4
                        (:Completed
                          (CallFunction|HUDStanimaHide)
                          (CallFunction|StopOutOfBreath))))))))))))))

(event EventBeginPlay
  ;[0 1 0] Set the reference to character and controller (copy Saeed)
  (bind _ascharacter_generic (Utilities|Casting|CastToCharacter_Generic (Components|GetOwner)))
  (bind _output_get (Variables|Default|SetCharacterRefrence _ascharacter_generic))
  (bind _asan_tppanim_blueprint (Utilities|Casting|CastToAN_TPPAnimBlueprint (Components|SkeletalMesh|GetAnimInstance (Variables|/Script/Engine.Character|GetMesh (Variables|Default|GetCharacterRefrence)))))
  (Variables|Default|SetTPP_AnimationBP _asan_tppanim_blueprint)
  (bind _asfppanim_blueprint (Utilities|Casting|CastToFPPAnimBlueprint (Components|SkeletalMesh|GetAnimInstance (Variables|/Game/Blueprint/Character_Generic.Character_Generic_C|GetFPP (Variables|Default|GetCharacterRefrence)))))
  (Variables|Default|SetFPP_Animation _asfppanim_blueprint)
  (bind _asplayer_controller_generic (Utilities|Casting|CastToPlayerController_Generic (Game|GetPlayerController 0)))
  (Variables|Default|SetControllerRefrence _asplayer_controller_generic)
  (bind _asthe_game_instance (Utilities|Casting|CastTotheGameInstance (Game|GetGameInstance)))
  (Variables|Default|SetGameInstance _asthe_game_instance)
  (Variables|Default|SetStartLoc (Transformation|GetSocketLocation (Variables|/Game/Blueprint/Character_Generic.Character_Generic_C|GetGUN_FPP _output_get) "Gun"))
  (Variables|Default|SetStartRot (Variables|/Script/Engine.SceneComponent|GetRelativeRotation (Variables|/Game/Blueprint/Character_Generic.Character_Generic_C|GetGUN_FPP _output_get))))

(fn StartCasingParticle
  (params (ActorComponentObjectRefrenceFPP :type Actor%20Component%20Object%20Reference) (Character :type Character%20Generic%20Object%20Reference) (ActorComponentObjectRefrenceTPP :type Actor%20Component%20Object%20Reference))
  (bind _currentweapon (Variables|/Game/Blueprint/Character_Generic.Character_Generic_C|GetCurrentWeapon Character))
  (bind _particlecasing (Utilities|Struct|BreakWeaponStruct _currentweapon))
  (Effects|Components|ParticleSystem|SetTemplate (Variables|/Game/Blueprint/Character_Generic.Character_Generic_C|GetBulletCasingEjectFPP Character) _particlecasing)
  (Effects|Components|ParticleSystem|SetTemplate (Variables|/Game/Blueprint/Character_Generic.Character_Generic_C|GetBulletCasingEjectTPP Character) _particlecasing)
  (Components|Activation|Activate ActorComponentObjectRefrenceFPP false)
  (return))

(fn StopCasingParticle
  (params (ActorComponentObjectRefrence :type Actor%20Component%20Object%20Reference) (Character :type Character%20Generic%20Object%20Reference))
  (Effects|Components|ParticleSystem|SetTemplate (Variables|/Game/Blueprint/Character_Generic.Character_Generic_C|GetBulletCasingEjectFPP Character) (.ParticleCasing (Utilities|Struct|BreakWeaponStruct (Variables|/Game/Blueprint/Character_Generic.Character_Generic_C|GetCurrentWeapon Character))))
  (Components|Activation|Deactivate ActorComponentObjectRefrence)
  (return))

(fn NormaltoRotator
  (params (InVec :type Vector))
  (bind (_x _y _z) (Math|Vector|BreakVector InVec))
  (return (Math|Rotator|MakeRotator (Class|KismetMathLibrary|DegAtan2 _y _z) (* (Class|KismetMathLibrary|DegAtan2 _x _z) -1.0) 0.0)))

(fn CasingBounceSound
  (params (Time :type Float%20%28single-precision%29%20%28by%20ref%29))
  (bind _characterrefrence (Variables|Default|GetCharacterRefrence))
  (if (and (not (<= (.AmmoInMag (Utilities|Struct|BreakWeaponStruct (Variables|/Game/Blueprint/Character_Generic.Character_Generic_C|GetCurrentWeapon _characterrefrence))) 0)) (Variables|/Game/Blueprint/Character_Generic.Character_Generic_C|GetIsFiring _characterrefrence))
    (Class|AkGameplayStatics|PostEvent "/Game/SoundWave/SFX/Weapons/AK47/Play_SFX_BulletCasingBounce.Play_SFX_BulletCasingBounce" (Game|GetPlayerCharacter 0) false)
    (Utilities|Time|SetTimerbyFunctionName 0 "MulticastBulletCasingBounce" Time true)
    (else
      (Utilities|Time|ClearTimerbyFunctionName 0 "MulticastBulletCasingBounce"))))

(fn StartMuzzleFlashParticle
  (params (ActorComponentObjectRefrenceFPP :type Actor%20Component%20Object%20Reference) (Character :type Character%20Generic%20Object%20Reference) (ActorComponentObjectRefrenceTPP :type Actor%20Component%20Object%20Reference))
  (bind _currentweapon (Variables|/Game/Blueprint/Character_Generic.Character_Generic_C|GetCurrentWeapon Character))
  (bind _particleflash (Utilities|Struct|BreakWeaponStruct _currentweapon))
  (Effects|Components|ParticleSystem|SetTemplate (Variables|/Game/Blueprint/Character_Generic.Character_Generic_C|GetMuzzleFlashFPP Character) _particleflash)
  (Effects|Components|ParticleSystem|SetTemplate (Variables|/Game/Blueprint/Character_Generic.Character_Generic_C|GetMuzzleFlashTPP Character) _particleflash)
  (Components|Activation|Activate ActorComponentObjectRefrenceFPP false)
  (return))

(fn StopMuzzleFlashParticle
  (params (ActorComponentObjectRefrence :type Actor%20Component%20Object%20Reference) (Character :type Character%20Generic%20Object%20Reference))
  (Effects|Components|ParticleSystem|SetTemplate (Variables|/Game/Blueprint/Character_Generic.Character_Generic_C|GetMuzzleFlashFPP Character) (.ParticleFlash (Utilities|Struct|BreakWeaponStruct (Variables|/Game/Blueprint/Character_Generic.Character_Generic_C|GetCurrentWeapon Character))))
  (Components|Activation|Deactivate ActorComponentObjectRefrence)
  (return))