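; Generic multiplayer player controller handling character spawning and respawning, player names, match timer state, scoring and HUD.
; Server requests spawn characters through GameMode_E1M1, while Tick copies that game mode's clock and countdown, hiding the countdown UI at zero.
; It scans all controllers to gather names, kills and deaths for an unfinished ranking, and to push kill-feed and winner widgets to each.
; Input actions add AI characters and show a respawn test menu.
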(event Custom|StartRespawnCountDown
  ;[0.07819 1 0.162] Player Respawn Countdown
  (Utilities|Time|SetTimerbyFunctionName self "RespawnCountdown" 1.0 true))

(event Custom|GetAllPlayerNames
  ;[0.1062 1 0.2026] Get all players names
  (Variables|Default|SetPlayerName (Variables|Default|GetNullArray))
  (bind _outactors (Actor|GetAllActorsOfClass "PlayerController_Generic_C"))
  (for _array_element _outactors
    (Utilities|Array|Add (Variables|Default|GetPlayerName) (Variables|PlayerController_Generic_C|GetPC_PlayerName _array_element))
    (Utilities|Array|Add (Variables|Default|GetPlayerName) (Variables|PlayerController_Generic_C|GetPC_ServerName _array_element)))
  (for (_array_element_2 _array_index) (Variables|Default|GetPlayerName)
    (if (Utilities|Text|TextIsEmpty _array_element_2)
      (Utilities|Array|RemoveIndex (Variables|Default|GetPlayerName) _array_index))))

(event Custom|MulticastRankingUpdate
  ;[1 1 1] Under process
  (Networking|SwitchHasAuthority
    (:Remote
      (Development|PrintString (Utilities|String|ToString(Integer) (Variables|Score|GetPosition)) true true "(R=0.000000,G=0.660000,B=1.000000,A=1.000000)" 1e+01))))

(event Custom|ControllerSetPlayerName
  (params (PlayerInfo :type Player%20Info%20Structure))
  ;[0.07819 1 0.162] Set Player Name
  (bind _asthe_game_instance (Utilities|Casting|CastTotheGameInstance (Game|GetGameInstance)))
  (Variables|/Game/Blueprint/AllLevels/theGameInstance.theGameInstance_C|SetPlayerSettings _asthe_game_instance PlayerInfo))

(event Custom|ShowWinner
  (params (winner :type Text))
  ;[0.08557 1 0.06308] Win  Conditions
  (Default|DisableInputsAllPlayers (Variables|GameObject|GetCharacterBP) self)
  (Utilities|IsValid (Variables|Default|GetWinnerRef)
    (:Is%20Valid
      (Widget|RemovefromParent (Variables|Default|GetWinnerRef)))
    (:Is%20Not%20Valid
      (bind _returnvalue (UserInterface|CreateWidget "/Game/Blueprint/Widgets/W_Winner.W_Winner_C" 0 winner))
      (bind _output_get (Variables|Default|SetWinnerRef _returnvalue))))
  (UserInterface|Viewport|AddtoViewport _output_get 10)
  (Variables|Default|SetbShowMouseCursor true))

(event Custom|Show%20Kill%20Feed%20on%20Server
  (params (killerIndex :type Integer) (victimIndex :type Integer))
  ;[0.07819 1 0.162] Show kill feed
  (bind _outactors (Actor|GetAllActorsOfClass "PlayerController_Generic_C"))
  (for (_array_element _array_index) _outactors
    (if (== (Variables|PlayerController_Generic_C|GetMyIndex _array_element) killerIndex)
      (bind _output_get (Variables|Default|SetlocalKiller (Utilities|Array|Get(acopy) (Variables|Default|GetPlayerName) _array_index)))))
  (bind _outactors_2 (Actor|GetAllActorsOfClass "PlayerController_Generic_C"))
  (for (_array_element_2 _array_index_2) _outactors_2
    (if (== (Variables|PlayerController_Generic_C|GetMyIndex _array_element_2) victimIndex)
      (bind _output_get_2 (Variables|Default|SetlocalVictim (Utilities|Array|Get(acopy) (Variables|Default|GetPlayerName) _array_index_2)))))
  (bind _outactors_3 (Actor|GetAllActorsOfClass "PlayerController_Generic_C"))
  (for _array_element_3 _outactors_3
    (CallFunction|KillFeedClient _array_element_3 _output_get _output_get_2)))

(event Custom|GetAllKills
  ;[0.1733 1 0.1562] Get all players kills
  (Utilities|Array|Clear (Variables|Score|GetPlayerKills))
  (bind _outactors (Actor|GetAllActorsOfClass "PlayerController_Generic_C"))
  (for _array_element _outactors
    (Utilities|Array|Add (Variables|Score|GetPlayerKills) (Variables|PlayerController_Generic_C|GetKills _array_element))))

(event Custom|kill%20feed%20Client
  (params (killer :type Text) (victim :type Text))
  ;[0.07819 1 0.162] Show kill feed
  (Utilities|IsValid (Variables|Default|Getw_killFeedRef)
    (:Is%20Valid
      (if (UserInterface|Viewport|IsinViewport (Variables|Default|Getw_killFeedRef))
        _
        (else
          (UserInterface|Viewport|AddtoViewport (stale _output_get) 5 :!label _label))))
    (:Is%20Not%20Valid
      (bind _returnvalue (UserInterface|CreateWidget "/Game/Blueprint/Widgets/W_KillFeed.W_KillFeed_C" (Game|GetPlayerController 0)))
      (bind _output_get (Variables|Default|Setw_killFeedRef _returnvalue))
      (goto _label)))
  (Default|GetPlayerKillerandVictim (Variables|Default|Getw_killFeedRef) killer victim))

(event Custom|AddPlayerNameServer
  (params (ServerName :type Text))
  ;[1 1 1] Server Name Oficial
  (Variables|PlayerInfo|SetPC_ServerName ServerName))

(event Custom|Run%20WinConditions%20OnServer
  ;[0.08557 1 0.06308] Win  Conditions
  (CallFunction|GetAllKills)
  (bind _asplayer_controller_generic (Utilities|Casting|CastToPlayerController_Generic (Game|GetPlayerController (.IndexOfMaxValue (Math|Integer|MaxOfIntArray (Variables|Score|GetPlayerKills))))))
  (if (Utilities|Text|TextIsEmpty (Variables|PlayerController_Generic_C|GetPC_ServerName _asplayer_controller_generic))
    (Variables|Default|Setwinner (Variables|PlayerController_Generic_C|GetPC_PlayerName _asplayer_controller_generic))
    (else
      (Variables|Default|Setwinner (Variables|PlayerController_Generic_C|GetPC_ServerName _asplayer_controller_generic))))
  (bind _outactors (Actor|GetAllActorsOfClass "PlayerController_Generic_C"))
  (for _array_element _outactors
    (CallFunction|ShowWinner _array_element (Variables|Default|Getwinner))))

(event Custom|AddPlayerNameClients
  (params (PlayerName :type Text))
  ;[1 1 1] Player Name Oficial
  (Variables|Player_Info|SetPC_PlayerName PlayerName))

(event Custom|GetAllDeath
  ;[0.1295 1 0.1096] Get all players death
  (Utilities|Array|Clear (Variables|Score|GetPlayerDeaths))
  (bind _outactors (Actor|GetAllActorsOfClass "PlayerController_Generic_C"))
  (for _array_element _outactors
    (Utilities|Array|Add (Variables|Score|GetPlayerDeaths) (Variables|PlayerController_Generic_C|GetDeath _array_element))))

(event Custom|RankingUpdate
  ;[1 1 1] Under process
  (Utilities|FlowControl|Sequence
    (:then_0
      (CallFunction|GetAllKills))
    (:then_1
      (CallFunction|Ranking)
      (Utilities|FlowControl|Delay 1.0))
    (:then_2
      (CallFunction|MulticastRankingUpdate))))

(event Custom|RespawnCountdown
  ;[0.07819 1 0.162] Player Respawn Countdown
  (if (== (Variables|Player-Respawn|GetRespawnCount) 0)
    (Utilities|Time|ClearTimerbyFunctionName self "RespawnCountdown")
    (Variables|Player-Respawn|SetRespawnCount (Variables|Player-Respawn|GetRespawnTime))
    (else
      (Variables|Player-Respawn|SetRespawnCount (- (Variables|Player-Respawn|GetRespawnCount) 1)))))

(event EventDestroyed
  (bind _thegamemode (Variables|GameObject|GetTheGameMode))
  ;[1 1 1] Controller Destroyed
  (Utilities|IsValid _thegamemode
    (:Is%20Valid
      (Utilities|Array|RemoveIndex (Variables|/Game/Blueprint/GameMode_E1M1.GameMode_E1M1_C|GetPlayerControllerArray _thegamemode) (Variables|GameObject|GetMyIndex))
      (Variables|/Game/Blueprint/GameMode_E1M1.GameMode_E1M1_C|SetPlayerCountNum _thegamemode (- (Variables|/Game/Blueprint/GameMode_E1M1.GameMode_E1M1_C|GetPlayerCountNum _thegamemode) 1)))))

(event EventBeginPlay
  ;[0.07819 1 0.162] After travel give the players the input back
  (Input|SetInputModeGameOnly self)
  ;[0.07819 1 0.162] Getting player Name from instance
  (bind _asthe_game_instance (Utilities|Casting|CastTotheGameInstance (Game|GetGameInstance)))
  (CallFunction|AddPlayerNameClients (Variables|/Game/Blueprint/AllLevels/theGameInstance.theGameInstance_C|GetPlayerName _asthe_game_instance))
  (CallFunction|AddPlayerNameServer (Variables|/Game/Blueprint/AllLevels/theGameInstance.theGameInstance_C|GetServerName _asthe_game_instance)))

(event EventTick
  (params (DeltaSeconds :type Float%20%28single-precision%29))
  ;[0.07819 1 0.162] Update Clock and Initial Countdown using GM
  (CallFunction|UpdatePCClock)
  (CallFunction|UpdatePCInitialCountdown)
  ;[0.07819 1 0.162] Remove Countdown UI
  (CallFunction|RemoveCountDownUI))

(event Input|ActionEvents|InputActionWinConditions
  (params (Key :type Key%20Structure))
  ;[0.08557 1 0.06308] Win  Conditions
)

(event Custom|RequestSpawnCharacterOnServer
  ;[0 1 0] Request Character Spawn On Server, it calls when player joins the game and want to be initiated
  (bind _asgame_mode_e1m1 (Utilities|Casting|CastToGameMode_E1M1 (Game|GetGameMode)))
  (bind _resultcharacter (Default|CreateNewCharacter _asgame_mode_e1m1 self "/Game/Blueprint/Character_Generic.Character_Generic_C"))
  (Utilities|IsValid _resultcharacter
    (:Is%20Valid
      (bind _output_get (Variables|GameObject|SetCharacterBP _resultcharacter))
      (Variables|/Game/Blueprint/Character_Generic.Character_Generic_C|SetPlController _output_get self))))

(event Custom|RequestRespawnCharacterOnServer
  ;[0 1 0] Request respawning the existing character
  (Utilities|IsValid (Variables|GameObject|GetCharacterBP)
    (:Is%20Valid
      (Actor|DestroyActor (Variables|GameObject|GetCharacterBP)))
    (:Is%20Not%20Valid
      _))
  (Utilities|IsValid (Variables|GameObject|GetTheGameMode)
    (:Is%20Valid
      _)
    (:Is%20Not%20Valid
      (bind _asgame_mode_e1m1 (Utilities|Casting|CastToGameMode_E1M1 (Game|GetGameMode)))
      (bind _output_get (Variables|GameObject|SetTheGameMode _asgame_mode_e1m1))))
  (bind _resultcharacter (Default|SpawnCharacter _output_get "/Game/Blueprint/Character_Generic.Character_Generic_C" (Variables|GameObject|GetMyIndex) self))
  (Utilities|IsValid _resultcharacter
    (:Is%20Valid
      (bind _output_get_2 (Variables|GameObject|SetCharacterBP _resultcharacter))
      (Variables|/Game/Blueprint/Character_Generic.Character_Generic_C|SetPlController _output_get_2 self)
      (bind _ashud_generic (Utilities|Casting|CastToHud_Generic (HUD|GetHUD)))
      (Variables|/Script/Engine.HUD|SetbShowHUD _ashud_generic true))))

(event Custom|RequestHUDClient
  ;[0.1436 1 0.0916] Add Request HUD for Client
  (Utilities|FlowControl|Sequence
    (:then_0
      (Viewport|RemoveAllWidgets))
    (:then_1
      (bind _asthe_game_instance (Utilities|Casting|CastTotheGameInstance (Game|GetGameInstance)))
      (Default|ShowHud _asthe_game_instance))))

(event Input|ActionEvents|InputActionAddRandomAI
  (params (Key :type Key%20Structure))
  ;[1 1 1] Add Random AI
  (:Pressed
    (bind _returnvalue (AI|SpawnAIFromClass "/Game/Blueprint/Character_Generic.Character_Generic_C" 0 (Transformation|GetActorLocation (Variables|GameObject|GetCharacterBP)) "0, 0, 0" true))
    (Utilities|IsValid _returnvalue
      (:Is%20Valid
        (Pawn|SpawnDefaultController _returnvalue)))))

(event Input|ActionEvents|InputActionRespawnTest
  (params (Key :type Key%20Structure))
  ;[1 1 1] Respawn widget
  (:Pressed
    (Viewport|RemoveAllWidgets)
    (bind _returnvalue (UserInterface|CreateWidget "/Game/Blueprint/Widgets/W_Main.W_Main_C" self))
    (UserInterface|Viewport|AddtoViewport _returnvalue 0)
    (bind _output_get (Variables|Default|SetLobbyWidget _returnvalue))
    (Variables|/Game/Blueprint/Widgets/W_Main.W_Main_C|SetuseFree4AllWidget _output_get true)
    (Variables|Default|SetbShowMouseCursor true))
  (:Released
    (Viewport|RemoveAllWidgets)
    (Variables|Default|SetbShowMouseCursor false)))

(fn ConstructionScript)

(fn MenuShow
  (params (MenuClass :type User%20Widget%20Class%20Reference))
  (Utilities|IsValid (Variables|Menu|GetScreenMenu)
    (:Is%20Valid
      (if (== (Utilities|GetClass (Variables|Menu|GetScreenMenu)) MenuClass)
        _
        (else
          (bind _returnvalue (UserInterface|CreateWidget MenuClass self :!label _label))
          (bind _output_get (Variables|Menu|SetScreenMenu _returnvalue)))))
    (:Is%20Not%20Valid
      (goto _label)))
  (UserInterface|Viewport|AddtoViewport _output_get 0)
  (Variables|/Script/Engine.PlayerController|SetbShowMouseCursor self true)
  (Variables|Menu|SetMenuIsOnScreen true))

(fn MenuHide
  (Widget|RemovefromParent (Variables|Menu|GetScreenMenu))
  (Variables|/Script/Engine.PlayerController|SetbShowMouseCursor self false)
  (Variables|Menu|SetMenuIsOnScreen false))

(fn UpdatePCClock
  (bind _asgame_mode_e1m1 (Utilities|Casting|CastToGameMode_E1M1 (Game|GetGameMode)))
  (LocalVariables|SetGM_Ref _asgame_mode_e1m1)
  (Variables|GM_Clock|SetPC_seconds (Variables|/Game/Blueprint/GameMode_E1M1.GameMode_E1M1_C|Getseconds (LocalVariables|GetGM_Ref)))
  (Variables|GM_Clock|SetPC_minutes (Variables|/Game/Blueprint/GameMode_E1M1.GameMode_E1M1_C|Getminutes (LocalVariables|GetGM_Ref)))
  (Variables|GM_Clock|SetPC_decimal_seconds (Variables|/Game/Blueprint/GameMode_E1M1.GameMode_E1M1_C|Getdecimal_seconds (LocalVariables|GetGM_Ref))))

(fn UpdatePCInitialCountdown
  (bind _asgame_mode_e1m1 (Utilities|Casting|CastToGameMode_E1M1 (Game|GetGameMode)))
  (bind _output_get (Variables|GMCountdown|SetPC_Countdown (Variables|/Game/Blueprint/GameMode_E1M1.GameMode_E1M1_C|Getcountdown _asgame_mode_e1m1)))
  (if (== _output_get 0)
    (Variables|GMCountdown|SetPC_GM_Started true)
    (else
      (Variables|GMCountdown|SetPC_GM_Started false))))

(fn RemoveCountDownUI
  (if (Variables|GMCountdown|GetPC_GM_Started)
    (Variables|GMCountdown|SetPC_GM_Started true)
    (bind _asthe_game_instance (Utilities|Casting|CastTotheGameInstance (Game|GetGameInstance)))
    (if (Utilities|IsValid (Variables|/Game/Blueprint/AllLevels/theGameInstance.theGameInstance_C|GetW_UI_HUD_Ref _asthe_game_instance))
      (Default|HideCountDownUI (Variables|/Game/Blueprint/AllLevels/theGameInstance.theGameInstance_C|GetW_UI_HUD_Ref _asthe_game_instance)))
    (else
      (Variables|GMCountdown|SetPC_GM_Started false)
      (return))))

(fn Ranking
  (bind _playerkills (Variables|Score|GetPlayerKills))
  (bind (_indexofmaxvalue _maxvalue) (Math|Integer|MaxOfIntArray _playerkills))
  (Utilities|Array|Clear (Variables|Score|GetPlayerKillSorted))
  (while (> (Utilities|Array|Length _playerkills) 0)
    (Utilities|Array|Add (Variables|Score|GetPlayerKillSorted) _maxvalue)
    (Utilities|Array|RemoveIndex _playerkills _indexofmaxvalue)
    (for (_array_element _array_index) (Variables|Score|GetPlayerKillSorted)
      (if (== _array_element (Variables|Score|GetKills))
        (switch int _array_index
          (:0
            (Variables|Score|SetPosition 1))
          (:1
            (Variables|Score|SetPosition 2))
          (:2
            (Variables|Score|SetPosition 3))
          (:3
            (Variables|Score|SetPosition 4))
          (:4
            (Variables|Score|SetPosition 5))
          (:5
            (Variables|Score|SetPosition 6))
          (:6
            (Variables|Score|SetPosition 7))
          (:7
            (Variables|Score|SetPosition 8)))
        (return)))))