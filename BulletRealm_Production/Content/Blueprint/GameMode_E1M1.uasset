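; Game mode for E1M1 that runs a timed free-for-all match and spawns player characters.
; A looping timer runs the start countdown, then Tick drives a Delay-paced digit clock that calls RunWinConditionsOnServer on player controller 0 at zero.
; CreateNewCharacter checks the player cap, then spawns on authority at a random saved PlayerStart transform, possessing and registering the controller.
; WinConditions and CreateNewAI are empty stubs, and kill-leader printing is disconnected.
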(event Custom|StartFree4AllTimer
  ;[0.3515 1 0.2705] Clock free 4 all , Done by Tauan
  (Utilities|FlowControl|Delay 1.0)
  (Variables|Clock|Setseconds (- (Variables|Clock|Getseconds) 1))
  (CallFunction|CheckifClockEnded)
  (if (== (Variables|Clock|Getseconds) -1)
    (Variables|Clock|Setdecimal_seconds (- (Variables|Clock|Getdecimal_seconds) 1))
    (Variables|Clock|Setseconds 9)
    (if (== (Variables|Clock|Getdecimal_seconds) -1)
      (Variables|Clock|Setminutes (- (Variables|Clock|Getminutes) 1))
      (Variables|Clock|Setdecimal_seconds 5)
      (Variables|Clock|Setseconds 9))))

(event Custom|WinConditions
  ;[1 1 1] Win Conditions
)

(event Custom|StartGame
  ;[0.3515 1 0.2705] Initial Countdown Free 4 All , Done by tauan
  (Utilities|Time|SetTimerbyFunctionName self "StartInitialCountdown" 1.0 true))

(event Custom|CheckIfClockEnded
  ;[0.3515 1 0.2705] Clock free 4 all , Done by Tauan
  (if (== (Variables|Clock|Getminutes) 0)
    (if (== (Variables|Clock|Getseconds) 0)
      (if (== (Variables|Clock|Getdecimal_seconds) 0)
        (Variables|Default|SetisFree4AllEnded true)
        (bind _asplayer_controller_generic (Utilities|Casting|CastToPlayerController_Generic (Game|GetPlayerController 0)))
        (Default|RunWinConditionsonServer _asplayer_controller_generic)))))

(event Custom|StartInitialCountdown
  ;[0.3515 1 0.2705] Initial Countdown Free 4 All , Done by tauan
  (if (<= (Variables|Clock|Getcountdown) 0)
    (Utilities|Time|ClearTimerbyFunctionName self "StartInitialCountdown")
    (Variables|Default|SetisFree4AllStarted true)
    (Variables|Clock|Setcountdown 0)
    (else
      (Variables|Clock|Setcountdown (- (Variables|Clock|Getcountdown) 1)))))

(event EventTick
  (params (DeltaSeconds :type Float%20%28single-precision%29))
  ;[0.3541 1 0.2819] Event Tick Using For Game Timer
  (if (not (Variables|Default|GetisFree4AllEnded))
    (if (Variables|Default|GetisFree4AllStarted)
      (CallFunction|StartFree4AllTimer))
    (else
      (CallFunction|WinConditions))))

(event EventBeginPlay
  ;[0.3515 1 0.2705] Initial Countdown Free 4 All , Done by tauan
  ;;[0.2602 1 0.2891] Begin Play - Starting clock
  (CallFunction|StartGame))

(fn ConstructionScript)

(fn SavePlayersStartPosition
  ;[1 1 1] Saving Player Start Positions
  (bind _outactors (Actor|GetAllActorsOfClass "/Script/Engine.PlayerStart"))
  (for _array_element _outactors
    (Utilities|Array|Add (Variables|Properties|GetARSaveStartPlayerPositions) (Transformation|GetActorTransform _array_element))))

(fn CreateNewPlayerIndex
  (if (<= (Variables|CurrentState|GetPlayerCountNum) (Variables|DefaultValue|GetPlayerMaxAllowed))
    (bind _output_get (Variables|CurrentState|SetPlayerCountNum (+ (Variables|CurrentState|GetPlayerCountNum) 1)))
    (return (<= (Variables|CurrentState|GetPlayerCountNum) (Variables|DefaultValue|GetPlayerMaxAllowed)) (- _output_get 1))))

(fn CreateNewCharacter
  (params (InputController :type Player%20Controller%20Generic%20Object%20Reference) (CharacterClass :type Character%20Generic%20Class%20Reference) (Controller :type Controller%20Object%20Reference))
  (bind (_creationallowed _playerindex) (CallFunction|CreateNewPlayerIndex))
  (if _creationallowed
    (bind _resultcharacter (CallFunction|SpawnCharacter CharacterClass _playerindex InputController))
    (return _resultcharacter)))

(fn SpawnCharacter
  (params (CharacterClass :type Character%20Generic%20Class%20Reference) (InputIndex :type Integer) (InputController :type Player%20Controller%20Generic%20Object%20Reference) (Controller :type Controller%20Object%20Reference))
  (bind _arsavestartplayerpositions (Variables|Properties|GetARSaveStartPlayerPositions))
  (Networking|SwitchHasAuthority
    (:Authority
      (bind _returnvalue (Game|SpawnActorfromClass CharacterClass (Utilities|Array|Get(acopy) _arsavestartplayerpositions (Math|Random|RandomIntegerinRange 0 (- (Utilities|Array|Length _arsavestartplayerpositions) 1))) "AlwaysSpawn" 0 0))
      (Utilities|IsValid _returnvalue
        (:Is%20Valid
          (Pawn|Possess InputController _returnvalue)
          (Variables|/Game/Blueprint/PlayerController_Generic.PlayerController_Generic_C|SetMyIndex InputController InputIndex)
          (Utilities|Array|Add (Variables|SpawnController|GetPlayerControllerArray) InputController)
          (return _returnvalue))))))

(fn CreateNewAI
  (params (InputController :type AI%20Controller%20Object%20Reference) (CharacterClass :type Character%20Generic%20Class%20Reference))
  (return 0))

(fn SendClocktoPC
  (params (minutes :type Integer) (seconds :type Integer) (decimal_seconds :type Integer))
  (bind _asplayer_controller_generic (Utilities|Casting|CastToPlayerController_Generic (Game|GetPlayerController 0)))
  (Variables|/Game/Blueprint/PlayerController_Generic.PlayerController_Generic_C|SetPC_minutes _asplayer_controller_generic minutes)
  (Variables|/Game/Blueprint/PlayerController_Generic.PlayerController_Generic_C|SetPC_seconds _asplayer_controller_generic seconds)
  (Variables|/Game/Blueprint/PlayerController_Generic.PlayerController_Generic_C|SetPC_decimal_seconds _asplayer_controller_generic decimal_seconds))