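; Character ability component for Character_Generic, handling shooting, reloading, melee, aiming and movement in a shooter.
; Server and multicast-named events drive ammo, timer-repeated projectile fire and melee actor spawning.
; Request checks gate melee, aim and movement, while sibling CharAbilities components supply stamina regeneration, montages, sounds and state checks.
; Crouch and sprint events are empty stubs with disconnected logic, and the IceBox graph holds unused movement and lean code.
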(event Custom|ServerStartCrouch
  ;[0 255 0] Crouch (Added crouch movement speed and camera by Hasan)(BUG: Character goes underground while crouching)
)

(event Custom|CancelMoveForward
  (bind _charref (Variables|Default|GetCharRef))
  ;[1 1 1] Movement (We need to return crouch/walking function if needed)
  ;;[1 1 1] Cancel / End MoveForward
  (Variables|/Game/Blueprint/Character_Generic.Character_Generic_C|SetIsMoving _charref false)
  (Variables|/Game/Blueprint/Character_Generic.Character_Generic_C|SetxAxis _charref 0.0))

(event Custom|GunFireEnd
  ;[0.1301 0.1221 0.4072] Server Release Fire > Multicast Fire Release
  (CallFunction|ServerRelesaeFire))

(event Custom|MulticastStartCrouch
  ;[0 255 0] Crouch (Added crouch movement speed and camera by Hasan)(BUG: Character goes underground while crouching)
)

(event Custom|ServerMeleeStart
  (bind _charref (Variables|Default|GetCharRef))
  ;[1 1 0] Melee attack under process
  (Variables|/Game/Blueprint/Character_Generic.Character_Generic_C|SetIsMelle _charref true)
  (bind _returnvalue (Game|SpawnActorfromClass "/Game/Blueprint/MeleeAttack.MeleeAttack_C" (Transformation|GetWorldTransform (Variables|/Game/Blueprint/Character_Generic.Character_Generic_C|GetcMeleeAttack _charref)) "AlwaysSpawn" _charref _charref))
  (Variables|/Game/Blueprint/MeleeAttack.MeleeAttack_C|SetCharacterOwner _returnvalue _charref)
  (Default|StartMeleeMontage (Variables|/Game/Blueprint/Character_Generic.Character_Generic_C|GetCharAbilities_DH _charref))
  (Class|AkGameplayStatics|PostEvent 0 (Variables|Default|GetCharRef) false)
  (Utilities|FlowControl|Delay (Variables|/Game/Blueprint/Character_Generic.Character_Generic_C|GetmonDurMelee (Variables|Default|GetCharRef)))
  (CallFunction|ServerMeleeEnd))

(event Custom|ServerAimCancel
  ;[0 0 1] Aiming done, but has unknown issues combining with the animations.
  (Variables|/Game/Blueprint/Character_Generic.Character_Generic_C|SetIsAiming (Variables|Default|GetCharRef) false))

(event Custom|ReleaseFireWhileReloadingMulticast
  ;[0.1301 0.1221 0.4072] Server Release Fire > Multicast Fire Release
  (Utilities|Time|PauseTimerbyHandle (Variables|Default|GetBulletSpawnTimer)))

(event Custom|AimingPressed
  (bind _charref (Variables|Default|GetCharRef))
  ;[0 0 1] Aiming done, but has unknown issues combining with the animations.
  (bind _answer (Default|AimRequested (Variables|/Game/Blueprint/Character_Generic.Character_Generic_C|GetCharAbilities_TB _charref)))
  (if _answer
    (Default|WeaponAim _charref)
    (CallFunction|ServerCancelSprint)
    (CallFunction|ServerAimStart)))

(event Custom|ServerMeleeEnd
  (bind _charref (Variables|Default|GetCharRef))
  ;[1 1 0] Melee attack under process
  (Variables|/Game/Blueprint/Character_Generic.Character_Generic_C|SetIsMelle _charref false)
  (bind (_isokay _state) (Default|CheckAfterMeleeNew (Variables|/Game/Blueprint/Character_Generic.Character_Generic_C|GetCharAbilities_SS _charref)))
  (if _isokay
    (switch int _state)))

(event Custom|StartSprint
  ;[1 0 0] Sprint done, need to be tested
)

(event Custom|ServerMeleeCancel
  (bind _charref (Variables|Default|GetCharRef))
  ;[1 1 0] Melee attack under process
  (Variables|/Game/Blueprint/Character_Generic.Character_Generic_C|SetIsMelle _charref false)
  (bind (_isokay _state) (Default|CheckAfterMeleeNew (Variables|/Game/Blueprint/Character_Generic.Character_Generic_C|GetCharAbilities_SS _charref)))
  (if _isokay
    (switch int _state)))

(event Custom|ServerAimStart
  (bind _charref (Variables|Default|GetCharRef))
  ;[0 0 1] Aiming done, but has unknown issues combining with the animations.
  (bind _answer (Default|AimRequested (Variables|/Game/Blueprint/Character_Generic.Character_Generic_C|GetCharAbilities_TB _charref)))
  (if _answer
    (Variables|/Game/Blueprint/Character_Generic.Character_Generic_C|SetIsAimingPressed _charref true)
    (Variables|/Game/Blueprint/Character_Generic.Character_Generic_C|SetIsAiming _charref true)
    (Default|Aim (Variables|/Game/Blueprint/CharAbilities_DH.CharAbilities_DH_C|GetTPP_AnimationBP (Variables|/Game/Blueprint/Character_Generic.Character_Generic_C|GetCharAbilities_DH _charref)))))

(event Custom|ServerGunFireStart
  (bind _charref (Variables|Default|GetCharRef))
  ;[0.4072 0.3763 0.05127] Gun fire under process
  (if (Variables|/Game/Blueprint/Character_Generic.Character_Generic_C|GetIsReloading _charref)
    (CallFunction|ReleaseFireWhileReloadingMulticast)
    (elif (> (Variables|/Game/Blueprint/Character_Generic.Character_Generic_C|GetAmmoInMag _charref) 0)
      (Variables|/Game/Blueprint/Character_Generic.Character_Generic_C|SetAmmoInMag _charref (- (Variables|/Game/Blueprint/Character_Generic.Character_Generic_C|GetAmmoInMag _charref) 1))
      (Variables|/Game/Blueprint/Character_Generic.Character_Generic_C|SetIsFiring _charref true)
      (CallFunction|MulticastGunFireStart)
      (Utilities|FlowControl|Delay (Variables|/Game/Blueprint/Character_Generic.Character_Generic_C|GetFiringDuration _charref))
      (else
        (CallFunction|ServerRelaseFireMulticast)
        (Default|EmptyAKSound (Variables|Default|GetCharAbilities_DH))))))

(event Custom|EndSprint
  ;[1 0 0] Sprint done, need to be tested
)

(event Custom|ReloadReleasedMulticast
  ;[0.2705 0.2451 1] Reload / Ammo Done by Hasan & Dean
  (Utilities|FlowControl|Delay 2.167)
  (Variables|/Game/Blueprint/Character_Generic.Character_Generic_C|SetIsReloading (stale Custom|ReloadMulticast _ascharacter_generic) false))

(event Custom|MoveForward
  (params (AxisValue :type Float%20%28single-precision%29))
  (bind _charref (Variables|Default|GetCharRef))
  (bind _charref_2 (Variables|Default|GetCharRef))
  (bind _charref_3 (Variables|Default|GetCharRef))
  ;[1 1 1] Movement (We need to return crouch/walking function if needed)
  ;;[1 1 1] Client Move Forward
  (if (!= AxisValue 0.0)
    (bind _answer (CallFunction|RunRequest))
    (if _answer
      (Variables|/Game/Blueprint/Character_Generic.Character_Generic_C|SetIsMovingPressed _charref_2 true)
      (Variables|/Game/Blueprint/Character_Generic.Character_Generic_C|SetIsMoving _charref_2 true)
      (Camera|PlayWorldCameraShake "/Game/Blueprint/CameraShakes/WalkCameraShake.WalkCameraShake_C" (Transformation|GetWorldLocation (Variables|/Game/Blueprint/Character_Generic.Character_Generic_C|GetFPSCamera (Variables|Default|GetCharRef))) 0.0 5e+01)
      ;;[1 1 1] Start Sprintring if holding shift
      (if (Variables|/Game/Blueprint/Character_Generic.Character_Generic_C|GetIsSprintingPressed _charref)
        (if (Variables|/Game/Blueprint/Character_Generic.Character_Generic_C|GetIsSprinting _charref)
          (Camera|PlayWorldCameraShake "/Game/Blueprint/CameraShakes/SprintCameraShake.SprintCameraShake_C" (Transformation|GetWorldLocation (Variables|/Game/Blueprint/Character_Generic.Character_Generic_C|GetFPSCamera _charref)) 0.0 5e+01)
          (else
            (Default|StartSprint (Variables|/Game/Blueprint/Character_Generic.Character_Generic_C|GetCharAbilities_SS _charref)))))
      (bind _output_get (Variables|/Game/Blueprint/Character_Generic.Character_Generic_C|SetxAxis _charref_3 AxisValue))
      (Pawn|Input|AddMovementInput _charref_3 (Math|Vector|GetForwardVector (Math|Rotator|MakeRotator 0.0 0.0 (.Yaw (Math|Rotator|BreakRotator (Pawn|GetControlRotation _charref_3 :!class /Script/Engine.Pawn))))) _output_get false))
    (else
      (Variables|/Game/Blueprint/Character_Generic.Character_Generic_C|SetIsMoving _charref_3 false))))

(event Custom|ServerAimEnd
  ;[0 0 1] Aiming done, but has unknown issues combining with the animations.
  (Variables|/Game/Blueprint/Character_Generic.Character_Generic_C|SetIsAimingPressed (Variables|Default|GetCharRef) false)
  (CallFunction|ServerAimCancel))

(event Custom|ServerStartSprint
  ;[1 0 0] Sprint done, need to be tested
)

(event Custom|MoveRight
  (params (Axis%20Value :type Float%20%28single-precision%29))
  (bind _charref (Variables|Default|GetCharRef))
  ;[1 1 1] Movement (We need to return crouch/walking function if needed)
  ;;[1 1 1] Client Move Right
  (if (!= Axis%20Value 0.0)
    (bind _answer (CallFunction|RunRequest))
    (if _answer
      (Variables|/Game/Blueprint/Character_Generic.Character_Generic_C|SetIsMovingPressed _charref true)
      (Variables|/Game/Blueprint/Character_Generic.Character_Generic_C|SetIsMoving _charref true)
      (Variables|/Game/Blueprint/Character_Generic.Character_Generic_C|SetyAxis _charref Axis%20Value)
      (Pawn|Input|AddMovementInput _charref (Math|Vector|GetRightVector (Math|Rotator|MakeRotator 0.0 0.0 (.Yaw (Math|Rotator|BreakRotator (Pawn|GetControlRotation _charref :!class /Script/Engine.Pawn))))) Axis%20Value false))
    (else
      (Variables|/Game/Blueprint/Character_Generic.Character_Generic_C|SetIsMoving _charref false))))

(event Custom|RequestReloadOnServer
  ;[0.2705 0.2451 1] Reload / Ammo Done by Hasan & Dean
  (CallFunction|ReloadMulticast))

(event Custom|MulticastEndCrouch
  ;[0 255 0] Crouch (Added crouch movement speed and camera by Hasan)(BUG: Character goes underground while crouching)
)

(event Custom|CancelMoveRight
  (bind _charref (Variables|Default|GetCharRef))
  ;[1 1 1] Movement (We need to return crouch/walking function if needed)
  ;;[1 1 1] Cancel / End MoveRight
  (Variables|/Game/Blueprint/Character_Generic.Character_Generic_C|SetIsMoving _charref false)
  (Variables|/Game/Blueprint/Character_Generic.Character_Generic_C|SetxAxis _charref 0.0))

(event Custom|MulticastGunFireStart
  (bind _charref (Variables|Default|GetCharRef))
  (bind _spherehead (Variables|/Game/Blueprint/Character_Generic.Character_Generic_C|GetSphereHead _charref))
  (bind _returnvalue (Transformation|GetWorldLocation _spherehead))
  ;[0.4072 0.3763 0.05127] Gun fire under process
  (Game|SpawnActorfromClass "/Game/Blueprint/Projectile_Generic.Projectile_Generic_C" (Math|Transform|MakeTransform _returnvalue (Math|Conversions|RotationFromXVector (- _returnvalue (Transformation|GetWorldLocation (Variables|/Game/Blueprint/Character_Generic.Character_Generic_C|GetSphereTail _charref))))) "AlwaysSpawn" 0 0))

(event Custom|RequestReloadReleaseOnServer
  ;[0.2705 0.2451 1] Reload / Ammo Done by Hasan & Dean
  (CallFunction|ReloadReleasedMulticast))

(event Custom|ServerEndSprint
  ;[1 0 0] Sprint done, need to be tested
)

(event Custom|Melee%20Pressed
  (bind _charref (Variables|Default|GetCharRef))
  (bind _charref_2 (Variables|Default|GetCharRef))
  (bind _charabilities_ss (Variables|/Game/Blueprint/Character_Generic.Character_Generic_C|GetCharAbilities_SS _charref_2))
  ;[1 1 0] Melee attack under process
  (bind _answer (Default|MeleeRequested (Variables|/Game/Blueprint/Character_Generic.Character_Generic_C|GetCharAbilities_TB (Variables|Default|GetCharRef))))
  (if _answer
    (Utilities|FlowControl|Sequence
      (:then_0
        (if (Variables|/Game/Blueprint/Character_Generic.Character_Generic_C|GetIsSprinting _charref_2)
          (Default|ServerCancelSprint _charabilities_ss))
        (if (Variables|/Game/Blueprint/Character_Generic.Character_Generic_C|GetIsFiring _charref_2)
          (Default|ServerGunFireCancel _charabilities_ss))
        (if (Variables|/Game/Blueprint/Character_Generic.Character_Generic_C|GetIsAiming _charref_2)
          (Default|AimCancel _charabilities_ss))
        (if (Variables|/Game/Blueprint/Character_Generic.Character_Generic_C|GetIsLeaningRightPressed _charref_2)
          (Default|LeanRightEnd _charref_2))
        (if (Variables|/Game/Blueprint/Character_Generic.Character_Generic_C|GetIsLeaningLeftPressed _charref_2)
          (Default|LeanLeftEnd _charref_2)))
      (:then_1
        (Variables|/Game/Blueprint/Character_Generic.Character_Generic_C|SetStamina _charref (- (Variables|/Game/Blueprint/Character_Generic.Character_Generic_C|GetStamina _charref) (Variables|/Game/Blueprint/Character_Generic.Character_Generic_C|GetStCostMelee _charref)))
        (if (Variables|/Game/Blueprint/Character_Generic.Character_Generic_C|GetIsSprinting _charref)
          _
          (else
            (Utilities|Time|ClearandInvalidateTimerbyHandle (Variables|/Game/Blueprint/Character_Generic.Character_Generic_C|GetTimerStaminaRegeneration _charref))
            (bind _returnvalue (Utilities|Time|SetTimerbyFunctionName (Variables|/Game/Blueprint/Character_Generic.Character_Generic_C|GetCharAbilities_SS _charref) "StaminaGenerate" (Variables|/Game/Blueprint/Character_Generic.Character_Generic_C|GetStCooldown _charref) true))
            (Variables|/Game/Blueprint/Character_Generic.Character_Generic_C|SetTimerStaminaRegeneration _charref _returnvalue)))
        (CallFunction|ServerMeleeStart)))))

(event Custom|ServerRelesaeFire
  ;[0.1301 0.1221 0.4072] Server Release Fire > Multicast Fire Release
  (Variables|/Game/Blueprint/Character_Generic.Character_Generic_C|SetIsFiring (Variables|Default|GetCharRef) false)
  (CallFunction|ServerRelaseFireMulticast))

(event Custom|ServerEndCrouch
  ;[0 255 0] Crouch (Added crouch movement speed and camera by Hasan)(BUG: Character goes underground while crouching)
)

(event Custom|EndMoveRight
  ;[1 1 1] Movement (We need to return crouch/walking function if needed)
  ;;[1 1 1] Cancel / End MoveRight
  (Variables|/Game/Blueprint/Character_Generic.Character_Generic_C|SetIsMovingPressed (Variables|Default|GetCharRef) false))

(event Custom|AimingReleased
  ;[0 0 1] Aiming done, but has unknown issues combining with the animations.
  (Default|HipAim (Variables|Default|GetCharRef))
  (CallFunction|ServerAimEnd))

(event Custom|GunFireStart
  (bind _charref (Variables|Default|GetCharRef))
  ;[0.4072 0.3763 0.05127] Gun fire under process
  (Utilities|Time|ClearandInvalidateTimerbyHandle (Variables|Default|GetBulletSpawnTimer))
  (if (not (Variables|/Game/Blueprint/Character_Generic.Character_Generic_C|GetIsReloading _charref))
    (if (> (Variables|/Game/Blueprint/Character_Generic.Character_Generic_C|GetAmmoInMag _charref) 0)
      (CallFunction|ServerGunFireStart)
      (bind _returnvalue (Utilities|Time|SetTimerbyEvent (EventDispatchers|CreateEvent :!event Custom|ServerGunFireStart) 0.1 true))
      (Variables|Default|SetBulletSpawnTimer _returnvalue)
      (CallFunction|MulticastGunFireStart)
      (Default|BulletCasingBounceSound (Variables|Default|GetCharAbilities_DH)))))

(event Custom|ServerRelaseFireMulticast
  ;[0.1301 0.1221 0.4072] Server Release Fire > Multicast Fire Release
  (if (not (Variables|/Game/Blueprint/Character_Generic.Character_Generic_C|GetIsReloading (Variables|Default|GetCharRef)))
    (Utilities|Time|PauseTimerbyHandle (Variables|Default|GetBulletSpawnTimer))))

(event Custom|ServerCancelSprint
  ;[1 0 0] Sprint done, need to be tested
)

(event Custom|CancelSprint
  ;[1 0 0] Sprint done, need to be tested
)

(event Custom|ReloadMulticast
  (bind _ascharacter_generic (Utilities|Casting|CastToCharacter_Generic (Components|GetOwner)))
  (if (> (Variables|/Game/Blueprint/Character_Generic.Character_Generic_C|GetTotalGunAmmo _ascharacter_generic) 0)
    (switch int (Variables|/Game/Blueprint/Character_Generic.Character_Generic_C|GetCurrentWeaponType _ascharacter_generic) ; 1= Primary, 2= Secondary, 3= Melee, 4= Grenade, 5= Tool
      (:1
        (if (< (Variables|/Game/Blueprint/Character_Generic.Character_Generic_C|GetAmmoInMag _ascharacter_generic) (Variables|/Game/Blueprint/Character_Generic.Character_Generic_C|GetAK47MaxMagAmmo _ascharacter_generic))
          (if (> (Variables|/Game/Blueprint/Character_Generic.Character_Generic_C|GetAK47Magazine _ascharacter_generic) 0)
            (Variables|/Game/Blueprint/Character_Generic.Character_Generic_C|SetIsReloading _ascharacter_generic true :!label _label)
            (if (not (Variables|/Game/Blueprint/Character_Generic.Character_Generic_C|GetIsAiming _ascharacter_generic))
              ;[0.2705 0.2451 1] Reload / Ammo Done by Hasan & Dean
              (if (Variables|/Game/Blueprint/Character_Generic.Character_Generic_C|GetGunCanReload _ascharacter_generic)
                (Utilities|FlowControl|Delay 2.167)
                (Variables|/Game/Blueprint/Character_Generic.Character_Generic_C|SetNeededAmmo _ascharacter_generic (- (Variables|/Game/Blueprint/Character_Generic.Character_Generic_C|GetMaxMagAmmo _ascharacter_generic) (Variables|/Game/Blueprint/Character_Generic.Character_Generic_C|GetAmmoInMag _ascharacter_generic)))
                (if (>= (Variables|/Game/Blueprint/Character_Generic.Character_Generic_C|GetTotalGunAmmo _ascharacter_generic) (Variables|/Game/Blueprint/Character_Generic.Character_Generic_C|GetNeededAmmo _ascharacter_generic))
                  (Variables|/Game/Blueprint/Character_Generic.Character_Generic_C|SetAmmoInMag _ascharacter_generic (+ (Variables|/Game/Blueprint/Character_Generic.Character_Generic_C|GetAmmoInMag _ascharacter_generic) (Variables|/Game/Blueprint/Character_Generic.Character_Generic_C|GetNeededAmmo _ascharacter_generic)))
                  (Variables|/Game/Blueprint/Character_Generic.Character_Generic_C|SetTotalGunAmmo _ascharacter_generic (- (Variables|/Game/Blueprint/Character_Generic.Character_Generic_C|GetTotalGunAmmo _ascharacter_generic) (Variables|/Game/Blueprint/Character_Generic.Character_Generic_C|GetNeededAmmo _ascharacter_generic)))
                  (switch int (Variables|/Game/Blueprint/Character_Generic.Character_Generic_C|GetCurrentWeaponType _ascharacter_generic) ; 1= Primary, 2= Secondary, 3= Melee, 4= Grenade, 5= Tool
                    (:1
                      (Variables|/Game/Blueprint/Character_Generic.Character_Generic_C|SetAK47Magazine _ascharacter_generic (Math|Integer|Clamp(Integer) (- (Variables|/Game/Blueprint/Character_Generic.Character_Generic_C|GetAK47Magazine _ascharacter_generic) 1) 0 5))
                      (if (Variables|/Game/Blueprint/Character_Generic.Character_Generic_C|GetIsAiming _ascharacter_generic)
                        _)))
                  (elif (> (Variables|/Game/Blueprint/Character_Generic.Character_Generic_C|GetTotalGunAmmo _ascharacter_generic) 0)
                    (Variables|/Game/Blueprint/Character_Generic.Character_Generic_C|SetAmmoInMag _ascharacter_generic (+ (Variables|/Game/Blueprint/Character_Generic.Character_Generic_C|GetAmmoInMag _ascharacter_generic) (Variables|/Game/Blueprint/Character_Generic.Character_Generic_C|GetTotalGunAmmo _ascharacter_generic)))
                    (Variables|/Game/Blueprint/Character_Generic.Character_Generic_C|SetTotalGunAmmo _ascharacter_generic 0))))))))
      (:2
        (if (< (Variables|/Game/Blueprint/Character_Generic.Character_Generic_C|GetAmmoInMag _ascharacter_generic) (Variables|/Game/Blueprint/Character_Generic.Character_Generic_C|GetFNP90MaxMagAmmo _ascharacter_generic))
          (goto _label))))))

(event Custom|StartCrouch
  ;[0 255 0] Crouch (Added crouch movement speed and camera by Hasan)(BUG: Character goes underground while crouching)
)

(event Custom|EndMoveForward
  ;[1 1 1] Movement (We need to return crouch/walking function if needed)
  ;;[1 1 1] Cancel / End MoveForward
  (Variables|/Game/Blueprint/Character_Generic.Character_Generic_C|SetIsMovingPressed (Variables|Default|GetCharRef) false))

(event Custom|EndCrouch
  ;[0 255 0] Crouch (Added crouch movement speed and camera by Hasan)(BUG: Character goes underground while crouching)
)

(event EventBeginPlay
  ;[0 1 0] Set the reference to character and controller
  (bind _ascharacter_generic (Utilities|Casting|CastToCharacter_Generic (Components|GetOwner)))
  (Variables|Default|SetCharRef _ascharacter_generic)
  (bind _asplayer_controller_generic (Utilities|Casting|CastToPlayerController_Generic (Game|GetPlayerController 0)))
  (Variables|Default|SetControllerRef _asplayer_controller_generic))

(event Custom|LeanRight)

(event Custom|ServerMoveRight
  (params (AxisValue :type Float%20%28single-precision%29))
  ;[1 1 1] Server Move Right
)

(event Custom|ServerMoveForward
  (params (AxisValue :type Float%20%28single-precision%29))
  ;[1 1 1] Server Move Forward
)

(fn RunRequest
  (bind _charref (Variables|Default|GetCharRef))
  (return (Math|Boolean|ANDBoolean (not (Variables|/Game/Blueprint/Character_Generic.Character_Generic_C|GetIsHealing _charref)) (not (AI|Components|NavMovement|IsFalling (Variables|/Script/Engine.Character|GetCharacterMovement _charref))) (not (Variables|/Game/Blueprint/Character_Generic.Character_Generic_C|GetIsMedLanding _charref)) (not (Variables|/Game/Blueprint/Character_Generic.Character_Generic_C|GetIsHitBySomething _charref)) (not (Variables|/Game/Blueprint/Character_Generic.Character_Generic_C|GetIsHigLanding _charref)))))

(fn CheckAfterSprint
  (bind _charref (Variables|Default|GetCharRef))
  (if (Variables|/Game/Blueprint/Character_Generic.Character_Generic_C|GetIsAimingPressed _charref)
    (Variables|/Game/Blueprint/Character_Generic.Character_Generic_C|SetIsAiming _charref true)
    (Variables|Default|SetSprintEndResult 1)
    (return (Variables|Default|GetSprintEndResult))))

(fn CheckAfterReload
  (if (Variables|/Game/Blueprint/Character_Generic.Character_Generic_C|GetIsAimingPressed (Variables|Default|GetCharRef))
    (Variables|Default|SetSprintEndResult 1)
    (return (Variables|Default|GetSprintEndResult))))

(fn CheckAfterSwitch
  (if (Variables|/Game/Blueprint/Character_Generic.Character_Generic_C|GetIsAimingPressed (Variables|Default|GetCharRef))
    (Variables|Default|SetSprintEndResult 1)
    (return (Variables|Default|GetSprintEndResult))))

(fn CheckAfterMelee
  (if (Variables|/Game/Blueprint/Character_Generic.Character_Generic_C|GetIsAimingPressed (Variables|Default|GetCharRef))
    (Variables|Default|SetSprintEndResult 1)
    (return (Variables|Default|GetSprintEndResult))))

(fn CheckAfterJump
  (if (Variables|/Game/Blueprint/Character_Generic.Character_Generic_C|GetIsAimingPressed (Variables|Default|GetCharRef))
    (Variables|Default|SetSprintEndResult 1)
    (return (Variables|Default|GetSprintEndResult))))

(fn CheckAfterLLand
  (if (Variables|/Game/Blueprint/Character_Generic.Character_Generic_C|GetIsAimingPressed (Variables|Default|GetCharRef))
    (Variables|Default|SetSprintEndResult 1)
    (return (Variables|Default|GetSprintEndResult))))

(fn CheckAfterMLand
  (if (Variables|/Game/Blueprint/Character_Generic.Character_Generic_C|GetIsAimingPressed (Variables|Default|GetCharRef))
    (Variables|Default|SetSprintEndResult 1)
    (return (Variables|Default|GetSprintEndResult))))

(fn CheckAfterHLand
  (if (Variables|/Game/Blueprint/Character_Generic.Character_Generic_C|GetIsAimingPressed (Variables|Default|GetCharRef))
    (Variables|Default|SetSprintEndResult 1)
    (return (Variables|Default|GetSprintEndResult))))

(fn CheckAfterHitStag
  (if (Variables|/Game/Blueprint/Character_Generic.Character_Generic_C|GetIsAimingPressed (Variables|Default|GetCharRef))
    (Variables|Default|SetSprintEndResult 1)
    (return (Variables|Default|GetSprintEndResult))))

(fn Staminaspend
  (bind _charref (Variables|Default|GetCharRef))
  (if (Math|Boolean|ANDBoolean (Variables|/Game/Blueprint/Character_Generic.Character_Generic_C|GetIsSprinting _charref) (>= (Variables|/Game/Blueprint/Character_Generic.Character_Generic_C|GetStamina _charref) 0.0) (> (Variables|/Game/Blueprint/Character_Generic.Character_Generic_C|GetxAxis _charref) 0.0))
    (Variables|/Game/Blueprint/Character_Generic.Character_Generic_C|SetStamina _charref (- (Variables|/Game/Blueprint/Character_Generic.Character_Generic_C|GetStamina _charref) (Variables|/Game/Blueprint/Character_Generic.Character_Generic_C|GetStCostSprint _charref)))
    (return)
    (else
      (Default|ServerEndSprint (Variables|/Game/Blueprint/Character_Generic.Character_Generic_C|GetCharAbilities_SS _charref)))))