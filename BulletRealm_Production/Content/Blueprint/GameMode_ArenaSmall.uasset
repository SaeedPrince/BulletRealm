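; GameMode_ArenaSmall is a game mode that spawns and possesses characters for players and AI in an arena.
; SavePlayersStartPosition caches PlayerStart transforms, and CreateNewCharacter takes the next index from a capped player counter.
; SpawnCharacter uses that index to spawn at a cached transform on authority, then possesses via PlayerController_Generic or AI_Generic.
; Both branches share the step setting the player controller's MyIndex, and CreateNewAI is an empty stub.
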(fn ConstructionScript)

(fn SavePlayersStartPosition
  ;[1 1 1] Saving Player Start Positions
  (bind _outactors (Actor|GetAllActorsOfClass "/Script/Engine.PlayerStart"))
  (for _array_element _outactors
    (Utilities|Array|Add (Variables|Properties|GetARSaveStartPlayerPositions) (Transformation|GetActorTransform _array_element))))

(fn CreateNewPlayerIndex
  (if (<= (Variables|CurrentState|GetPlayerCountNum) (Variables|DefaultValue|GetPlayerMaxAllowed))
    (bind _output_get (Variables|CurrentState|SetPlayerCountNum (+ (Variables|CurrentState|GetPlayerCountNum) 1)))
    (return (<= (Variables|CurrentState|GetPlayerCountNum) (Variables|DefaultValue|GetPlayerMaxAllowed)) (- _output_get 1))))

(fn CreateNewCharacter
  (params (InputController :type Player%20Controller%20Object%20Reference) (CharacterClass :type Character%20Generic%20Class%20Reference) (Controller :type Controller%20Object%20Reference))
  (bind (_creationallowed _playerindex) (CallFunction|CreateNewPlayerIndex))
  (if _creationallowed
    (bind _resultcharacter (CallFunction|SpawnCharacter CharacterClass _playerindex 0 Controller))
    (return _resultcharacter)))

(fn SpawnCharacter
  (params (CharacterClass :type Character%20Generic%20Class%20Reference) (InputIndex :type Integer) (InputController :type Player%20Controller%20Object%20Reference) (Controller :type Controller%20Object%20Reference))
  (bind _returnvalue (Utilities|GetClass Controller))
  (Utilities|IsValid Controller
    (:Is%20Valid
      (Networking|SwitchHasAuthority
        (:Authority
          (bind _returnvalue_2 (Game|SpawnActorfromClass CharacterClass (Utilities|Array|Get(acopy) (Variables|Properties|GetARSaveStartPlayerPositions) InputIndex) "Undefined" Controller 0))
          (Utilities|IsValid _returnvalue_2
            (:Is%20Valid
              (if (== _returnvalue "/Game/Blueprint/PlayerController_Generic.PlayerController_Generic_C")
                (bind _asplayer_controller_generic (Utilities|Casting|CastToPlayerController_Generic Controller))
                (Pawn|Possess _asplayer_controller_generic _returnvalue_2)
                (Variables|/Game/Blueprint/PlayerController_Generic.PlayerController_Generic_C|SetMyIndex _asplayer_controller_generic InputIndex :!label _label)
                (return _returnvalue_2)
                (elif (== _returnvalue "/Game/Blueprint/AI_Generic.AI_Generic_C")
                  (bind _asai_generic (Utilities|Casting|CastToAI_Generic Controller))
                  (Pawn|Possess _asai_generic _returnvalue_2)
                  (goto _label))))))))))

(fn CreateNewAI
  (params (InputController :type AI%20Controller%20Object%20Reference) (CharacterClass :type Character%20Generic%20Class%20Reference))
  (return 0))