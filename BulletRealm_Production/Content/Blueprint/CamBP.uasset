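; CamBP is a camera Blueprint that keeps its camera component following the owning character's mesh while that character is not aiming.
; Each Tick it sets the camera's world transform from the mesh location plus an unrotated world-space offset and the mesh rotation combined with a rotation adjustment.
; The move is immediate, without interpolation or sweep, and camera scale is preserved.
; While the character aims, this Blueprint leaves the camera untouched.
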(event EventTick
  (params (DeltaSeconds :type Float%20%28single-precision%29))
  (bind _charowner (Variables|Character|GetCharOwner))
  (bind _mesh (Variables|/Script/Engine.Character|GetMesh _charowner))
  (bind _returnvalue (Transformation|GetWorldTransform _mesh))
  (bind (_location _rotation) (Math|Transform|BreakTransform _returnvalue))
  (if (not (Variables|/Game/Blueprint/Character_Generic.Character_Generic_C|GetIsAiming _charowner))
    (Transformation|SetWorldTransform (Variables|CameraActor|GetCameraComponent) (Math|Transform|MakeTransform (+ _location (Variables|Adjustment|GetLocationAdjustment)) (Math|Rotator|CombineRotators _rotation (Variables|Adjustment|GetRotationAdjustment)) (.Scale (Math|Transform|BreakTransform (Transformation|GetWorldTransform (Variables|CameraActor|GetCameraComponent))))) false false)))

(fn ConstructionScript)