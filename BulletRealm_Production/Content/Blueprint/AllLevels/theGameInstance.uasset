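; Game instance for a multiplayer game with an FFA lobby, acting as the central hub for UI and sessions.
; Show events lazily create and cache menu, HUD and feedback widgets, with a few matching hide events.
; It creates sessions and opens the listen lobby, joins the first LAN session found, and destroys the session on restart.
; Save-game checking is work in progress, and network error handlers are unwired.
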(event Custom|LaunchLobby
  (params (NumberOfPlayers :type Integer) (EnableLan? :type Boolean) (ServerName :type Text))
  (bind _w_hostref (Variables|Default|Getw_HostRef))
  ;[0.07843 1 0.1608] Launch Lobby
  (Variables|ServerSettings|SetMaxPlayer NumberOfPlayers)
  (Variables|ServerSettings|SetServerName ServerName)
  (Default|ShowCreatingGameUI (Variables|Default|Getw_HostRef))
  (Utilities|FlowControl|Delay 3.0)
  (|Session (Game|GetPlayerController 0) (Variables|ServerSettings|GetMaxPlayer) EnableLan?
    (:OnSuccess
      (Default|ResetHostUI _w_hostref)
      (Game|OpenLevel(byName) "FFA_Lobby" true "listen"))
    (:OnFailure
      (Default|ResetHostUI _w_hostref))))

(event Custom|ShowRespawnScreen
  ;[0.07819 1 0.162] Show w_Respawn
  (Utilities|IsValid (Variables|Default|Getw_RespawnScreen)
    (:Is%20Valid
      (if (not (UserInterface|Viewport|IsinViewport (Variables|Default|Getw_RespawnScreen)))
        (UserInterface|Viewport|AddtoViewport (stale _output_get) 10 :!label _label)))
    (:Is%20Not%20Valid
      (bind _returnvalue (UserInterface|CreateWidget "/Game/Blueprint/Widgets/W_Respawn.W_Respawn_C" (Game|GetPlayerController 0)))
      (bind _output_get (Variables|Default|Setw_RespawnScreen _returnvalue))
      (goto _label))))

(event Custom|ShowJoinMenu
  ;[0.07819 1 0.162] Show w_Joinlobby
  (Utilities|IsValid (Variables|Default|Getw_JoinLobbyRef)
    (:Is%20Valid
      _)
    (:Is%20Not%20Valid
      (bind _returnvalue (UserInterface|CreateWidget "/Game/Blueprint/Widgets/W_JoinLobby.W_JoinLobby_C" (Game|GetPlayerController 0)))
      (bind _output_get (Variables|Default|Setw_JoinLobbyRef _returnvalue))))
  (UserInterface|Viewport|AddtoViewport _output_get 0))

(event Custom|Show%20KillFeed
  ;[0.0865 1 0.2086] Show kill feed
  (Utilities|IsValid (Variables|Default|Getw_killFeedRef)
    (:Is%20Valid
      (if (not (UserInterface|Viewport|IsinViewport (Variables|Default|Getw_killFeedRef)))
        (UserInterface|Viewport|AddtoViewport (stale _output_get) 5 :!label _label)))
    (:Is%20Not%20Valid
      (bind _returnvalue (UserInterface|CreateWidget "/Game/Blueprint/Widgets/W_KillFeed.W_KillFeed_C" (Game|GetPlayerController 0)))
      (bind _output_get (Variables|Default|Setw_killFeedRef _returnvalue))
      (goto _label))))

(event Custom|SetGameResolution
  (params (PlayerControllerRef :type Player%20Controller%20Object%20Reference) (ResolutionInput :type String))
  ;[0.07843 1 0.1608] Set Resolution Screen
  (Development|ExecuteConsoleCommand ResolutionInput PlayerControllerRef))

(event Custom|Show%20w_hit
  ;[0.0865 1 0.2086] Show w_hit
  (Utilities|IsValid (Variables|Default|Getw_hitRef)
    (:Is%20Valid
      (if (not (UserInterface|Viewport|IsinViewport (Variables|Default|Getw_hitRef)))
        (UserInterface|Viewport|AddtoViewport (stale _output_get) 5 :!label _label)))
    (:Is%20Not%20Valid
      (bind _returnvalue (UserInterface|CreateWidget "/Game/Blueprint/Widgets/W_Hit.W_Hit_C" (Game|GetPlayerController 0)))
      (bind _output_get (Variables|Default|Setw_hitRef _returnvalue))
      (goto _label))))

(event Custom|Hide%20w_LowHealth
  (bind _w_lowhealthref (Variables|Default|Getw_LowHealthRef))
  ;[0.07819 1 0.162] Hide w_lowHealth
  (Utilities|IsValid _w_lowhealthref
    (:Is%20Valid
      (Widget|RemovefromParent _w_lowhealthref))))

(event Custom|Hide%20w_reloadFB
  (bind _w_reloadfbref (Variables|Default|Getw_ReloadFBRef))
  ;[0.07819 1 0.162] hide w_reloadFB
  (Utilities|IsValid _w_reloadfbref
    (:Is%20Valid
      (Widget|RemovefromParent _w_reloadfbref))))

(event Custom|Show%20w_Healing
  ;[0.07819 1 0.162] Show w_healingFeedback
  (Utilities|IsValid (Variables|Default|Getw_HealingRef)
    (:Is%20Valid
      (if (not (UserInterface|Viewport|IsinViewport (Variables|Default|Getw_HealingRef)))
        (UserInterface|Viewport|AddtoViewport (stale _output_get) 10 :!label _label)
        (Utilities|FlowControl|Delay 2.0)
        (Default|HealingStop (stale _output_get))
        (Widget|RemovefromParent (stale _output_get))))
    (:Is%20Not%20Valid
      (bind _returnvalue (UserInterface|CreateWidget "/Game/Blueprint/Widgets/W_Healing.W_Healing_C" (Game|GetPlayerController 0)))
      (bind _output_get (Variables|Default|Setw_HealingRef _returnvalue))
      (goto _label))))

(event Custom|Show%20w_lowHealth
  ;[0.07819 1 0.162] Show w_lowHealth
  (Utilities|IsValid (Variables|Default|Getw_LowHealthRef)
    (:Is%20Valid
      (if (not (UserInterface|Viewport|IsinViewport (Variables|Default|Getw_LowHealthRef)))
        (UserInterface|Viewport|AddtoViewport (stale _output_get) 15 :!label _label)))
    (:Is%20Not%20Valid
      (bind _returnvalue (UserInterface|CreateWidget "/Game/Blueprint/Widgets/W_LowHealth.W_LowHealth_C" (Game|GetPlayerController 0)))
      (bind _output_get (Variables|Default|Setw_LowHealthRef _returnvalue))
      (goto _label))))

(event Custom|RestartMatch
  ;[1 1 1] Restart the Match
  (|DestroySession (Game|GetPlayerController 0)
    (:then
      (Game|OpenLevel(byName) "Level_Entry" true "listen"))))

(event Custom|JoinLobby
  (params (PlayerName :type Text))
  ;[0.07843 1 0.1608] Join Lobby
  (Variables|PlayerInfo|SetPlayerName PlayerName)
  (Default|ShowJoiningUI (Variables|Default|Getw_JoinLobbyRef))
  (bind _results (|FindSessions (Game|GetPlayerController 0) 1 true)
    (:OnSuccess
      (if (> (Utilities|Array|Length _results) 0)
        (|JoinSession (Game|GetPlayerController 0) (Utilities|Array|Get(acopy) _results))
        (else
          (Development|PrintString "failed to find session")
          (Default|ResetJoiningUI (Variables|Default|Getw_JoinLobbyRef))
          (Viewport|RemoveAllWidgets)
          (Game|OpenLevel(byName) "Level_Entry"))))
    (:OnFailure
      (Development|PrintString "failed to find session"))))

(event Custom|Show%20w_ReloadFB
  ;[0.07819 1 0.162] show w_reloadFB
  (Utilities|IsValid (Variables|Default|Getw_ReloadFBRef)
    (:Is%20Valid
      (if (not (UserInterface|Viewport|IsinViewport (Variables|Default|Getw_ReloadFBRef)))
        (UserInterface|Viewport|AddtoViewport (stale _output_get) 10 :!label _label)))
    (:Is%20Not%20Valid
      (bind _returnvalue (UserInterface|CreateWidget "/Game/Blueprint/Widgets/W_ReloadFB.W_ReloadFB_C" (Game|GetPlayerController 0)))
      (bind _output_get (Variables|Default|Setw_ReloadFBRef _returnvalue))
      (goto _label))))

(event Custom|ShowEscapeMenu
  (bind _returnvalue (Game|GetPlayerController 0))
  (bind _wingamemenuref (Variables|Default|GetWInGameMenuRef))
  ;[0.07843 1 0.1608] Show Escape Game Menu
  (Utilities|IsValid _wingamemenuref
    (:Is%20Valid
      (if (UserInterface|Viewport|IsinViewport _wingamemenuref)
        _
        (else
          (UserInterface|Viewport|AddtoViewport (stale _output_get) 0 :!label _label))))
    (:Is%20Not%20Valid
      (bind _returnvalue_2 (UserInterface|CreateWidget "/Game/Blueprint/Widgets/W_InGameOptions.W_InGameOptions_C" _returnvalue))
      (bind _output_get (Variables|Default|Setw_inGameOptionsRef _returnvalue_2))
      (goto _label)))
  (Variables|/Script/Engine.PlayerController|SetbShowMouseCursor _returnvalue true))

(event Custom|Show%20w_HealingCooldownTime
  ;[0.07819 1 0.162] Show w_healingcooldown
  (Utilities|IsValid (Variables|Default|Getw_HealingCooldownTimeRef)
    (:Is%20Valid
      (if (not (UserInterface|Viewport|IsinViewport (Variables|Default|Getw_HealingCooldownTimeRef)))
        (UserInterface|Viewport|AddtoViewport (stale _output_get) 10 :!label _label)))
    (:Is%20Not%20Valid
      (bind _returnvalue (UserInterface|CreateWidget "/Game/Blueprint/Widgets/W_HealingCooldown.W_HealingCooldown_C" (Game|GetPlayerController 0)))
      (bind _output_get (Variables|Default|Setw_HealingCooldownTimeRef _returnvalue))
      (goto _label))))

(event Custom|Show%20w_Scoreboard
  ;[0.07819 1 0.162] Show w_scoreboard
  (Utilities|IsValid (Variables|Default|Getw_ScoreboardRef)
    (:Is%20Valid
      (if (not (UserInterface|Viewport|IsinViewport (Variables|Default|Getw_ScoreboardRef)))
        (UserInterface|Viewport|AddtoViewport (stale _output_get) 10 :!label _label)))
    (:Is%20Not%20Valid
      (bind _returnvalue (UserInterface|CreateWidget "/Game/Blueprint/Widgets/W_Scoreboard.W_Scoreboard_C" (Game|GetPlayerController 0)))
      (bind _output_get (Variables|Default|Setw_ScoreboardRef _returnvalue))
      (goto _label))))

(event Custom|ShowHud
  (bind _returnvalue (Game|GetPlayerController 0))
  ;[0.07819 1 0.162] Show Hud
  (Utilities|IsValid (Variables|Default|GetW_UI_HUD_Ref)
    (:Is%20Valid
      (if (UserInterface|Viewport|IsinViewport (Variables|Default|GetW_UI_HUD_Ref))
        _
        (else
          (UserInterface|Viewport|AddtoViewport (stale _output_get) 0 :!label _label))))
    (:Is%20Not%20Valid
      (bind _returnvalue_2 (UserInterface|CreateWidget "/Game/Blueprint/Widgets/UI_HUD_Widget.UI_HUD_Widget_C" _returnvalue))
      (bind _output_get (Variables|Default|SetW_UI_HUD_Ref _returnvalue_2))
      (goto _label)))
  (Variables|/Script/Engine.PlayerController|SetbShowMouseCursor _returnvalue false))

(event Custom|ShowMainMenu
  (bind _returnvalue (Game|GetPlayerController 0))
  ;[0.07819 1 0.162] 2.2 [True] Show w_EntryMenu
  (Utilities|IsValid (Variables|Widgets|GetMainMenuRef)
    (:Is%20Valid
      _)
    (:Is%20Not%20Valid
      (bind _returnvalue_2 (UserInterface|CreateWidget "/Game/Blueprint/Widgets/W_EntryMenu.W_EntryMenu_C" _returnvalue))
      (Variables|Widgets|SetMainMenuRef _returnvalue_2)))
  (UserInterface|Viewport|AddtoViewport (Variables|Widgets|GetMainMenuRef) 0)
  (Variables|/Script/Engine.PlayerController|SetbShowMouseCursor _returnvalue true))

(event Custom|CheckForSaveGame
  ;[0.07843 1 0.1608] 2. Check for Save Game - Work in Progress
  (bind _returnvalue (SaveGame|DoesSaveGameExist (Variables|Default|GetPlayerSettingsSave)))
  (if _returnvalue
    _
    (else
      (CallFunction|SaveforSupportSettings)))
  (CallFunction|ShowMainMenu)
  (Variables|Default|SetCreatedSaveFile? true))

(event Custom|Hide%20w_Scoreboard
  (bind _w_scoreboardref (Variables|Default|Getw_ScoreboardRef))
  ;[0.07819 1 0.162] Hide w_Score board
  (Utilities|IsValid _w_scoreboardref
    (:Is%20Valid
      (Widget|RemovefromParent _w_scoreboardref))))

(event Custom|ShowHostMenu
  ;[0.07843 1 0.1608] Show w_Host
  (Utilities|IsValid (Variables|Default|Getw_HostRef)
    (:Is%20Valid
      _)
    (:Is%20Not%20Valid
      (bind _returnvalue (UserInterface|CreateWidget "/Game/Blueprint/Widgets/W_Host.W_Host_C" (Game|GetPlayerController 0)))
      (bind _output_get (Variables|Default|Setw_HostRef _returnvalue))))
  (UserInterface|Viewport|AddtoViewport _output_get 0))

(event Custom|ShowCreditsMenu
  ;[0.07819 1 0.162] Show w_Credits
  (Utilities|IsValid (Variables|Default|Getw_Credits)
    (:Is%20Valid
      _)
    (:Is%20Not%20Valid
      (bind _returnvalue (UserInterface|CreateWidget "/Game/Blueprint/Widgets/W_Credits.W_Credits_C" (Game|GetPlayerController 0)))
      (bind _output_get (Variables|Default|Setw_Credits _returnvalue))))
  (UserInterface|Viewport|AddtoViewport _output_get 0))

(event Custom|SaveForSupportSettings
  (bind _savename (Variables|Default|GetSaveName))
  ;[0.07843 1 0.1608] 2.1[False] Create a save game object
  (bind _returnvalue (SaveGame|DoesSaveGameExist _savename))
  (if _returnvalue
    (bind _returnvalue_2 (SaveGame|LoadGamefromSlot _savename))
    (bind _asbp_save_game (Utilities|Casting|CastToBP_SaveGame _returnvalue_2))
    (Variables|Default|SetSaveGameRef _asbp_save_game)
    (else
      (bind _returnvalue_3 (SaveGame|CreateSaveGameObject "/Game/Blueprint/AllLevels/BP_SaveGame.BP_SaveGame_C"))
      (Variables|Default|SetSaveGameRef _returnvalue_3))))

(event EventHandleNetworkError
  (params (FailureType :type ENetworkFailure%20Enum :default "NetDriverAlreadyExists") (bIsServer :type Boolean))
  ;[0.08327 1 0.1783] Network Error Messages
)

(event EventHandleTravelError
  (params (FailureType :type ETravelFailure%20Enum :default "NoLevel"))
  ;[0.08327 1 0.1783] Network Error Messages
)