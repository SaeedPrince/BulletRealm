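; Weapon Blueprint that applies the stat preset for the AK47 or FN P90 to the character's active gun variables.
; Each gun has its own function that passes hardcoded damage and projectile speeds, plus that gun's ammo counts read from CharacterBP, into SetWeaponStats.
; The shared SetWeaponStats event writes these values back to CharacterBP as its current damage, ammo and projectile settings.
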(event Custom|SetWeaponStats
  (params (Damage :type Float%20%28single-precision%29) (MaxMagAmmo :type Integer) (TotalGunAmmo :type Integer) (ProjectileMaxSpeed :type Float%20%28single-precision%29) (ProjectileInitialSpeed :type Float%20%28single-precision%29) (AmmoInMag :type Integer))
  (bind _characterbp (Variables|Default|GetCharacterBP))
  (Variables|/Game/Blueprint/Character_Generic.Character_Generic_C|SetAmmoInMag _characterbp AmmoInMag)
  (Variables|/Game/Blueprint/Character_Generic.Character_Generic_C|SetBulletDamage _characterbp Damage)
  (Variables|/Game/Blueprint/Character_Generic.Character_Generic_C|SetMaxMagAmmo _characterbp MaxMagAmmo)
  (Variables|/Game/Blueprint/Character_Generic.Character_Generic_C|SetTotalGunAmmo _characterbp TotalGunAmmo)
  (Variables|/Game/Blueprint/Character_Generic.Character_Generic_C|SetProjectileMaxSpeed _characterbp ProjectileMaxSpeed)
  (Variables|/Game/Blueprint/Character_Generic.Character_Generic_C|SetProjectileInitialSpeed _characterbp ProjectileInitialSpeed))

(fn AK47
  (bind _characterbp (Variables|Default|GetCharacterBP))
  (CallFunction|SetWeaponStats 2e+01 (Variables|/Game/Blueprint/Character_Generic.Character_Generic_C|GetAK47MaxMagAmmo _characterbp) (Variables|/Game/Blueprint/Character_Generic.Character_Generic_C|GetAK47TotalGunAmmo _characterbp) 3e+03 3e+03 (Variables|/Game/Blueprint/Character_Generic.Character_Generic_C|GetAK47AmmoInMag _characterbp)))

(fn FNP90
  (bind _characterbp (Variables|Default|GetCharacterBP))
  (CallFunction|SetWeaponStats 12.0 (Variables|/Game/Blueprint/Character_Generic.Character_Generic_C|GetFNP90MaxMagAmmo _characterbp) (Variables|/Game/Blueprint/Character_Generic.Character_Generic_C|GetFNP90TotalGunAmmo _characterbp) 1e+03 1e+03 (Variables|/Game/Blueprint/Character_Generic.Character_Generic_C|GetFNP90AmmoInMag _characterbp)))