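; Cookable grenade actor that, on the server, detonates after the fuse time left from player 0's cooking.
; Detonation freezes the mesh, triggers the character's explosion sound, grows a damage sphere by timeline, then destroys the actor.
; A separate Hit event applies radial damage with falloff, radial force and camera shake before destroying it.
; The sphere's tiered overlap damage and the explosion-particle multicast call are disconnected.
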(event OnComponentBeginOverlap(GrenadeDamageSphere)
  (params (OverlappedComponent :type Primitive%20Component%20Object%20Reference) (OtherActor :type Actor%20Object%20Reference) (OtherComp :type Primitive%20Component%20Object%20Reference) (OtherBodyIndex :type Integer) (bFromSweep :type Boolean) (SweepResult :type Hit%20Result%20Structure%20%28by%20ref%29))
  ;[1 1 1] must go to icebox
)

(event Custom|PlaySound
  (params (ActorLocation :type Vector))
  ;[1 1 1] play explode sound at location after detonation time
)

(event Custom|MulticastDetonateGrenade
  ;[0.4072 0.3763 0.05127] Detonation under process by Saeed
  (Rendering|SetVisibility (Variables|Default|GetGrenadeMesh) false false)
  (Effects|SpawnEmitteratLocation "/Game/Particle/P_GrenadeExplosion.P_GrenadeExplosion" (Transformation|GetWorldLocation (Variables|Default|GetGrenadeMesh)) "0, 0, 0" false))

(event Custom|ServerDetonateGrenade
  (bind _grenadedamagesphere (Variables|Default|GetGrenadeDamageSphere))
  (bind _characterref (Variables|GameObject|GetCharacterRef))
  ;[0.4072 0.3763 0.05127] Detonation under process by Saeed
  (Utilities|IsValid _characterref
    (:Is%20Valid
      (Utilities|FlowControl|Sequence
        (:then_0
          (Variables|Calculation|SetDelayBeforeDetonate (- (- (- (Variables|/Game/Blueprint/Character_Generic.Character_Generic_C|GetCookingGrenadeDuration _characterref) (Variables|GameObject|GetBeginPlayDelayRequirement)) (Variables|/Game/Blueprint/Character_Generic.Character_Generic_C|GetGrenadeTimePass _characterref)) 1.0)))
        (:then_1
          (Utilities|Time|ClearandInvalidateTimerbyHandle (Variables|/Game/Blueprint/Character_Generic.Character_Generic_C|GetGrenadeTimer _characterref))
          (Variables|/Game/Blueprint/Character_Generic.Character_Generic_C|SetGrenadeTimePass _characterref 0.0)
          (Utilities|FlowControl|Delay (Variables|Calculation|GetDelayBeforeDetonate))
          (Utilities|FlowControl|Sequence
            (:then_0
              (Variables|State|SetIsDamaging true))
            (:then_1
              (Physics|SetSimulatePhysics (Variables|Default|GetGrenadeMesh) false)
              (Physics|SetEnableGravity (Variables|Default|GetGrenadeMesh) false))
            (:then_2
              (CallFunction|GrenadeSoundQue))
            (:then_3
              (Physics|SetSimulatePhysics _grenadedamagesphere false)
              (bind _radiussize (Timeline|GrenadeSphere PlayFromStart)
                (:Update
                  (Components|Sphere|SetSphereRadius _grenadedamagesphere (Math|Float|Lerp (Variables|/Script/Engine.SphereComponent|GetSphereRadius (Variables|Default|GetGrenadeDamageSphere)) (Variables|/Game/Blueprint/Character_Generic.Character_Generic_C|GetGrenadeRadius3 _characterref) _radiussize) true))))
            (:then_4
              (Utilities|FlowControl|Delay (Variables|/Game/Blueprint/Character_Generic.Character_Generic_C|GetDamagingDuration _characterref))
              (Variables|State|SetIsDamaging false)
              (Actor|DestroyActor))))))))

(event Custom|MulticastWallDamage
  (params (InputComponent :type Destructible%20Component%20Object%20Reference) (InputLocation :type Vector))
  (bind _characterref (Variables|GameObject|GetCharacterRef))
  ;[0.4072 0.3763 0.05127] Detonation under process by Saeed
  (Class|DestructibleComponent|ApplyRadiusDamage InputComponent (Variables|/Game/Blueprint/Character_Generic.Character_Generic_C|GetGrenadeDamage3 _characterref) InputLocation (Variables|/Game/Blueprint/Character_Generic.Character_Generic_C|GetGrenadeRadius3 _characterref) (Variables|/Game/Blueprint/Character_Generic.Character_Generic_C|GetGrenadeImpulseStrength _characterref) false))

(event EventBeginPlay
  ;[0.4072 0.3763 0.05127] Detonation under process by Saeed
  (bind _ascharacter_generic (Utilities|Casting|CastToCharacter_Generic (Game|GetPlayerCharacter 0)))
  (Variables|GameObject|SetCharacterRef _ascharacter_generic)
  (Utilities|FlowControl|Delay (Variables|GameObject|GetBeginPlayDelayRequirement))
  (Networking|SwitchHasAuthority
    (:Authority
      (CallFunction|ServerDetonateGrenade))))

(event Collision|EventHit
  (params (MyComp :type Primitive%20Component%20Object%20Reference) (Other :type Actor%20Object%20Reference) (OtherComp :type Primitive%20Component%20Object%20Reference) (bSelfMoved :type Boolean) (HitLocation :type Vector :default "0, 0, 0") (HitNormal :type Vector :default "0, 0, 0") (NormalImpulse :type Vector :default "0, 0, 0") (Hit :type Hit%20Result%20Structure%20%28by%20ref%29))
  (bind _characterref (Variables|GameObject|GetCharacterRef))
  (bind _characterref_2 (Variables|GameObject|GetCharacterRef))
  ;[0.4072 0.3763 0.05127] Grenade radial damage by Hasan
  (Game|SpawnActorfromClass "/Game/Blueprint/GrenadeRadialForce.GrenadeRadialForce_C" (Math|Transform|MakeTransform HitLocation) "Undefined" 0 0)
  (bind _returnvalue (Class|GameplayStatics|ApplyRadialDamagewithFalloff (Variables|/Game/Blueprint/Character_Generic.Character_Generic_C|GetGreandeBaseDamage _characterref_2) (Variables|/Game/Blueprint/Character_Generic.Character_Generic_C|GetGrenadeMinimumDamage _characterref_2) (Transformation|GetActorLocation) (Variables|/Game/Blueprint/Character_Generic.Character_Generic_C|GetGrenadeInnerRadius _characterref_2) (Variables|/Game/Blueprint/Character_Generic.Character_Generic_C|GetGrenadeOuterRadius _characterref_2) (Variables|/Game/Blueprint/Character_Generic.Character_Generic_C|GetGrenadeDamageFalloff _characterref_2) "/Script/Engine.DamageType" 0 self (Game|GetInstigatorController) "ECC_Visibility"))
  (Development|PrintString (Utilities|String|ToString(Boolean) _returnvalue))
  (Camera|PlayWorldCameraShake "/Game/Blueprint/CameraShakes/GrenadeCameraShake.GrenadeCameraShake_C" (Transformation|GetActorLocation) (Variables|/Game/Blueprint/Character_Generic.Character_Generic_C|GetGrenadeCameraShakeInnerRadius _characterref) (Variables|/Game/Blueprint/Character_Generic.Character_Generic_C|GetGrenadeCameraShakeOuterRadius _characterref) (Variables|/Game/Blueprint/Character_Generic.Character_Generic_C|GetGrenadeCameraShakeFalloff _characterref) true)
  (Actor|DestroyActor))

(fn ConstructionScript)

(fn IsAlreadyDamaged
  (params (ActorInput :type Actor%20Object%20Reference))
  (bind _array_element (Utilities|Array|ForEachLoopwithBreak (Variables|Hit|GetDamagedActors) :!label _label)
    (:LoopBody
      (if (== _array_element ActorInput)
        (LocalVariables|SetResult true)
        (goto _label Break)
        (else
          (LocalVariables|SetResult false))))
    (:Completed
      (return (LocalVariables|GetResult)))))

(fn GrenadeSoundQue
  (Default|MulticastGrenadeExplode (Variables|/Game/Blueprint/Character_Generic.Character_Generic_C|GetCharAbilities_DH (Variables|GameObject|GetCharacterRef)) self))