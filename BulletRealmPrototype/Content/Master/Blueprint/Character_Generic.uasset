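; Generic first-person shooter character with movement, firing, crouch, sprint, health and a HUD.
; Input calls server events that, by their names, multicast fire, crouch and sprint state, while projectiles spawn from the camera's aim.
; Sprint stamina drains and refills through self-rescheduling timers that pause each other.
; Damage lowers health and physics-simulates bodies below BoneName for dismemberment, though this file never sets that bone, and both crouch states use identical capsule height.
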(event Custom|ServerApplyDmgMulti
  (params (Damage :type Float%20%28single-precision%29))
  (bind _bonename (Variables|Physics|GetBoneName))
  (bind _mesh (Variables|Character|GetMesh))
  ;[1 1 1] Server Apply damage and dismembering
  (bind _output_get (Variables|Attribute|SetHealth (- (Variables|Attribute|GetHealth) Damage)))
  (Development|PrintString (Utilities|String|ToString(Float) _output_get) true false "(R=0.000000,G=0.660000,B=1.000000,A=1.000000)" 8.0)
  (Class|SkeletalMeshComponent|SetAllBodiesBelowSimulatePhysics _mesh _bonename true true)
  (Class|SkeletalMeshComponent|SetAllBodiesBelowPhysicsBlendWeight _mesh _bonename 1.0 false true)
  (Physics|AddForce _mesh "100.000000,100.000000,0.000000" _bonename false))

(event Custom|ServerApplyDamage
  (params (Damage :type Float%20%28single-precision%29))
  ;[1 1 1] Server Apply damage and dismembering
  (CallFunction|ServerApplyDmgMulti Damage))

(event Game|Damage|EventAnyDamage
  (params (Damage :type Float%20%28single-precision%29) (DamageType :type Damage%20Type%20Object%20Reference) (InstigatedBy :type Controller%20Object%20Reference) (DamageCauser :type Actor%20Object%20Reference))
  ;[1 1 1] Server Apply damage and dismembering
  (CallFunction|ServerApplyDamage Damage))

(event EventBeginPlay
  ;[1 1 1] Adding hud to view
  (CallFunction|AddHud))

(event Input|ActionEvents|InputActionSprint
  (params (Key :type Key%20Structure :default "AnyKey"))
  ;[1 1 1] Sprint
  (:Pressed
    (CallFunction|ServerSprintReplication))
  (:Released
    (CallFunction|ServerSprintRelease)))

(event Input|ActionEvents|InputActionFire
  (params (Key :type Key%20Structure :default "AnyKey"))
  ;[1 1 1] Fire
  (:Pressed
    (CallFunction|ServerFireReplicate)
    (CallFunction|SpawnProjectileonServer))
  (:Released
    (CallFunction|ServerRelesaeFire)))

(event Input|ActionEvents|InputActionCrouch
  (params (Key :type Key%20Structure :default "AnyKey"))
  ;[1 1 1] Crouch replication
  (:Pressed
    (CallFunction|ServerCrouchReplication))
  (:Released
    (CallFunction|ServerCrouchRelease)))

(event Input|AxisEvents|InputAxisTurn
  (params (AxisValue :type Float%20%28single-precision%29))
  ;[1 1 1] Character rotation
  (Pawn|Input|AddControllerYawInput AxisValue))

(event Input|AxisEvents|InputAxisLookUp
  (params (AxisValue :type Float%20%28single-precision%29))
  ;[1 1 1] Character rotation
  (Pawn|Input|AddControllerPitchInput AxisValue))

(event Input|AxisEvents|InputAxisMoveForward
  (params (AxisValue :type Float%20%28single-precision%29))
  ;[1 1 1] Character Movement
  (if (!= AxisValue 0.0)
    (Variables|Movement|SetxAxis AxisValue)
    (Pawn|Input|AddMovementInput (Math|Vector|GetForwardVector (Math|Rotator|MakeRotator 0.0 0.0 (.Yaw (Math|Rotator|BreakRotator (Pawn|GetControlRotation :!class /Script/Engine.Pawn))))) AxisValue false)
    (else
      (Variables|Movement|SetxAxis 0.0))))

(event Input|AxisEvents|InputAxisMoveRight
  (params (AxisValue :type Float%20%28single-precision%29))
  ;[1 1 1] Character Movement
  (Pawn|Input|AddMovementInput (Math|Vector|GetRightVector (Math|Rotator|MakeRotator 0.0 0.0 (.Yaw (Math|Rotator|BreakRotator (Pawn|GetControlRotation :!class /Script/Engine.Pawn))))) AxisValue false))

(event Custom|SpawnProjectileOnServer
  (bind _fpscamera (Variables|Default|GetFPSCamera))
  (bind _returnvalue (Transformation|GetWorldRotation _fpscamera))
  ;[1 1 1] Spawn Bullet on Server
  (Game|SpawnActorfromClass "/Game/Master/Blueprint/Projectile_Generic.Projectile_Generic_C" (Math|Transform|MakeTransform (+ (Transformation|GetWorldLocation (Variables|Default|GetSphere)) (Math|Vector|RotateVector (Variables|Projectile|GetGunOffset) _returnvalue)) _returnvalue) "Undefined" 0 0))

(event Custom|ServerMulticastFire
  ;[1 1 1] Fire Replication
  (Variables|State|SetIsFiring true)
  (Variables|Recoile|SetRecoileX (Math|Random|RandomFloatinRange -1e+02 1e+02))
  (Variables|Recoile|SetRecoileY (Math|Random|RandomFloatinRange -1e+02 1e+02))
  ;;[1 1 1] if gun was fired reduce the bullet count
  (Variables|Weapon|SetGunAmmo (Math|Integer|Clamp(Integer) (- (Variables|Weapon|GetGunAmmo) 1) 0 1000))
  (CallFunction|SetGunAmmo))

(event Custom|ServerMultCrouchRelease
  ;[1 0.88 0] Crouch
  (Variables|State|SetIsCrouching false)
  (Components|Capsule|SetCapsuleHalfHeight (Variables|Collision|GetCapsuleComponent) 96.0 true))

(event Custom|ServerCrouchRelease
  ;[1 0.88 0] Crouch
  (CallFunction|ServerMultCrouchRelease))

(event Custom|ServerFireReplicate
  ;[1 1 1] Fire Replication
  (CallFunction|ServerMulticastFire))

(event Custom|ServerRelesaeFire
  ;[1 1 1] Fire Replication
  (CallFunction|ServerRelaseFireMulticast))

(event Custom|ServerCrouchReplication
  ;[1 0.88 0] Crouch
  (CallFunction|ServerMulticastCrouchReplication))

(event Custom|ServerRelaseFireMulticast
  ;[1 1 1] Fire Replication
  (Variables|State|SetIsFiring false))

(event Custom|ServerSprintReplication
  ;[1 1 1] Sprint
  (CallFunction|ServerMultiSrpint))

(event Custom|ServerMulticastCrouchReplication
  ;[1 0.88 0] Crouch
  (Variables|State|SetIsCrouching true)
  (Components|Capsule|SetCapsuleHalfHeight (Variables|Collision|GetCapsuleComponent) 96.0 true))

(event Custom|ServerMultiSrpint
  ;[1 1 1] Sprint
  (CallFunction|ReduceStamina (>= (Math|Vector|VectorLength (Variables|/Script/Engine.MovementComponent|GetVelocity (Variables|Character|GetCharacterMovement))) 4e+02) 2.0 0.1))

(event Custom|ServerSprintRelease
  ;[1 1 1] Sprint
  (CallFunction|ServerMultiRelease))

(event Custom|ServerMultiRelease
  ;[1 1 1] Sprint
  (CallFunction|IncreaseStamina 1.0 0.3))

(event EventTick
  (params (DeltaSeconds :type Float%20%28single-precision%29))
  ;[1 1 1] Print Stamina and Sprinting
  (Development|PrintString (Utilities|String|ToString(Float) (Variables|Attribute|GetStamina)) true true "(R=0.021231,G=1.000000,B=0.000000,A=1.000000)" 0.0)
  (Development|PrintString (Utilities|String|ToString(Float) (Variables|/Script/Engine.CharacterMovementComponent|GetMaxWalkSpeed (Variables|Character|GetCharacterMovement))) true true "(R=1.000000,G=0.000000,B=0.091003,A=1.000000)" 0.0))

(fn ConstructionScript)

(fn SetGunAmmo
  (bind _gunammo (Variables|Weapon|GetGunAmmo))
  (Rendering|Components|TextRender|SetText (Variables|Default|GetAmmoCount) (Utilities|Text|ToText(Integer) (Math|Integer|Clamp(Integer) _gunammo 0 1000)))
  (if (<= _gunammo 0)
    (Variables|Weapon|SetEmptyAmmo? true)
    (else
      (Variables|Weapon|SetEmptyAmmo? false))))

(fn ReduceStamina
  (params (Condition :type Boolean) (Reduceamount :type Float%20%28single-precision%29) (Delay :type Float%20%28single-precision%29))
  (bind _self self)
  (Class|KismetSystemLibrary|PauseTimer _self "ServerMultiRelease")
  (Variables|State|SetIsSprinting true)
  (Variables|/Script/Engine.CharacterMovementComponent|SetMaxWalkSpeed (Variables|Character|GetCharacterMovement) 5e+03)
  (if Condition
    (Variables|Attribute|SetStamina (Math|Float|Clamp(Float) (- (Variables|Attribute|GetStamina) Reduceamount) 0.0 1e+02)))
  (Utilities|Time|SetTimerbyFunctionName _self "ServerMultiSrpint" Delay)
  (if (<= (Variables|Attribute|GetStamina) 0.0)
    (Class|KismetSystemLibrary|PauseTimer _self "ServerMultiSrpint")
    (Variables|/Script/Engine.CharacterMovementComponent|SetMaxWalkSpeed (Variables|Character|GetCharacterMovement) 6e+02)
    (else
      (return))))

(fn IncreaseStamina
  (params (increaseAmount :type Float%20%28single-precision%29) (Delay :type Float%20%28single-precision%29))
  (bind _self self)
  (Class|KismetSystemLibrary|PauseTimer _self "ServerMultiSrpint")
  (Variables|State|SetIsSprinting false)
  (Variables|/Script/Engine.CharacterMovementComponent|SetMaxWalkSpeed (Variables|Character|GetCharacterMovement) 6e+02)
  (Variables|Attribute|SetStamina (Math|Float|Clamp(Float) (+ (Variables|Attribute|GetStamina) increaseAmount) 0.0 1e+02))
  (Utilities|Time|SetTimerbyFunctionName _self "ServerMultiRelease" Delay)
  (if (>= (Variables|Attribute|GetStamina) 1e+02)
    (Class|KismetSystemLibrary|PauseTimer _self "ServerMultiRelease")))

(fn AddHud
  (bind _returnvalue (UserInterface|CreateWidget "/Game/UI/UI_HUD_Widget.UI_HUD_Widget_C" (Game|GetPlayerController 0)))
  (bind _output_get (Variables|Hud|SetPlayerWigetHUD _returnvalue))
  (UserInterface|Viewport|AddtoViewport _output_get 0))